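; Actor component that manages the equipped weapon of its owning GAS character.
; Equipping a different class replaces the current weapon, attaches the new actor to a mesh socket, and applies its config's granted abilities, anim class and walk speed.
; Unequipping destroys the weapon, removes those abilities and restores the default anim class and speed.
; When the owner is BP_Player, equipping also triggers a weapon save through GI_Global.
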(event `self.ReceiveBeginPlay`
  (bind _asgascharacter_base (cast `GASCharacterBase` (`self.GetOwner`)))
  (set `self.GASCharacter` _asgascharacter_base))

(event `EquipWeapon`
  (params (WeaponClass :type "/Game/Dynamic/Blueprints/Weapons/BP_Weapon_Base Class Reference"))
  (bind _gascharacter (`self.GASCharacter`))
  (bind _gascharacter_2 (`self.GASCharacter`)
    (:`then`
      (bind _equippedweapon (`self.EquippedWeapon`)
        (:`then`
          (if (not (== (`GameplayStatics.GetObjectClass` _equippedweapon) WeaponClass))
            (`self.UnequipWeapon`)
            (bind _returnvalue (`|SpawnActorFromClass` WeaponClass (`KismetMathLibrary.MakeTransform` (0.0 0.0 0.0)) "Undefined" "MultiplyWithRoot" null (`self.GASCharacter`) :!label _label))
            (bind _output_get (set `self.EquippedWeapon` _returnvalue))
            (bind _mesh (`Character.Mesh` _gascharacter_2))
            (bind ((`EquippedSocketName_5_FB6D3F2843F1A8CAD971D3A2D183A126` _equippedsocketname) (`AnimClass_8_75595F7D48FDB5F433F3FC9C9C21BF15` _animclass) (`MovementSpeed_11_004DA0D54D5750023D2F309C6BE2CDE0` _movementspeed)) (break `/Game/Dynamic/Blueprints/Weapons/Data/Str_WeaponConfig` (`/Game/Dynamic/Blueprints/Weapons/BP_Weapon_Base.WeaponConfig` _output_get)))
            (`Actor.K2_AttachToComponent` _output_get _mesh _equippedsocketname "SnapToTarget" "SnapToTarget" "SnapToTarget" true)
            (bind _returnvalue_2 (`GASCharacterBase.GrantAbilities` (`self.GASCharacter`) (`.AbilitiesToGrant_12_B0A255A54E15E9DB706062B3840B674A` (break `/Game/Dynamic/Blueprints/Weapons/Data/Str_WeaponConfig` (`/Game/Dynamic/Blueprints/Weapons/BP_Weapon_Base.WeaponConfig` (`self.EquippedWeapon`))))))
            (set `self.AbilitiesGrantedByWeapon` _returnvalue_2)
            (`SkeletalMeshComponent.SetAnimInstanceClass` _mesh _animclass)
            (set `CharacterMovementComponent.MaxWalkSpeed` _movementspeed (`Character.CharacterMovement` _gascharacter))
            (set `GASCharacterBase.hasWeaponEquipped` true _gascharacter)
            (bind _asbp_player (cast `/Game/Dynamic/Blueprints/Controllers/Player/BP_Player` (`self.GASCharacter`)))
            (`/Game/Dynamic/Blueprints/Controllers/Player/BP_Player.GetPlayerSave` _asbp_player)
            (bind _asgi_global (cast `/Game/Dynamic/Blueprints/SaveGame/GI_Global` (`GameplayStatics.GetGameInstance`)))
            (`/Game/Dynamic/Blueprints/SaveGame/GI_Global.SavePlayerWeapon` _asgi_global)))
        (:`else`
          (goto _label))))
    (:`else`)))

(event `UnequipWeapon`
  (bind _gascharacter (`self.GASCharacter`))
  (bind _gascharacter_2 (`self.GASCharacter`))
  (bind ((`AbilitiesToGrant_12_B0A255A54E15E9DB706062B3840B674A` _abilitiestogrant) (`AnimClass_8_75595F7D48FDB5F433F3FC9C9C21BF15` _animclass) (`MovementSpeed_11_004DA0D54D5750023D2F309C6BE2CDE0` _movementspeed)) (break `/Game/Dynamic/Blueprints/Weapons/Data/Str_WeaponConfig` (`self.DefaultWeaponConfig`)))
  (bind _equippedweapon (`self.EquippedWeapon`)
    (:`then`
      (`Actor.K2_DestroyActor` _equippedweapon)
      (`GASCharacterBase.RemoveAbilities` _gascharacter (`self.AbilitiesGrantedByWeapon`))
      (set `self.EquippedWeapon` null)
      (`SkeletalMeshComponent.SetAnimInstanceClass` (`Character.Mesh` _gascharacter) _animclass)
      (set `CharacterMovementComponent.MaxWalkSpeed` _movementspeed (`Character.CharacterMovement` _gascharacter_2))
      (set `GASCharacterBase.hasWeaponEquipped` false _gascharacter_2))
    (:`else`)))