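; Interactable pickup area that equips a weapon on the player or, when no weapon is set, grants the dash ability.
; A sphere overlap with the player shows and hides a press-F prompt widget.
; Interact sends the Event.Weapon.Equip gameplay event carrying the weapon's tag, or gives GA_Dash once and notifies the character that abilities changed.
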(event `self.ReceiveBeginPlay`
  (bind _returnvalue (`|CreateWidget` "/Game/Dynamic/Blueprints/WidgetBlueprint(WBP)/Prototype/WBP_PressF.WBP_PressF_C"))
  (set `self.Widget` _returnvalue)
  (set `self.DashEquipped?` false))

(event `/Game/Dynamic/Blueprints/InteractibleSystem/Interfaces/BPI_Interaction.Interact`
  (bind _weapontoequip (`self.WeaponToEquip`)
    (:`then`
      (`AbilitySystemBlueprintLibrary.SendGameplayEventToActor` (`GameplayStatics.GetPlayerCharacter` 0) (struct :`TagName` "Event.Weapon.Equip") (make `GameplayEventData` :`TargetTags` (`/Game/Dynamic/Blueprints/Weapons/BP_Weapon_Base.WeaponTag` _weapontoequip))))
    (:`else`
      (if (not (`self.DashEquipped?`))
        (`AbilitySystemComponent.K2_GiveAbility` (`AbilitySystemBlueprintLibrary.GetAbilitySystemComponent` (`GameplayStatics.GetPlayerPawn` 0)) "/Game/Dynamic/Blueprints/GameplayAbilitySystem/Abilities/Dash/GA_Dash.GA_Dash_C" 0 -1)
        (`GASCharacterBase.SendAbilitiesChangedEvent` (cast `GASCharacterBase` (`GameplayStatics.GetPlayerCharacter` 0) :!pure true))
        (set `self.DashEquipped?` true)))))

(event `self.Sphere.OnComponentBeginOverlap`
  (params (OverlappedComponent :type "PrimitiveComponent Object Reference") (OtherActor :type "Actor Object Reference") (OtherComp :type "PrimitiveComponent Object Reference") (OtherBodyIndex :type Integer) (bFromSweep :type Boolean) (SweepResult :type "HitResult Structure (by ref)"))
  (cast `/Game/Dynamic/Blueprints/Controllers/Player/BP_Player` OtherActor)
  (`UserWidget.AddToViewport` (`self.Widget`) 0))

(event `self.Sphere.OnComponentEndOverlap`
  (params (OverlappedComponent :type "PrimitiveComponent Object Reference") (OtherActor :type "Actor Object Reference") (OtherComp :type "PrimitiveComponent Object Reference") (OtherBodyIndex :type Integer))
  (cast `/Game/Dynamic/Blueprints/Controllers/Player/BP_Player` OtherActor)
  (`Widget.RemoveFromParent` (`self.Widget`)))

(fn `UserConstructionScript`)