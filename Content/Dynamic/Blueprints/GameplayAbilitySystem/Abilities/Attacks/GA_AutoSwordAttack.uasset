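; Gameplay ability that makes the player automatically swing a sword every second while enemies are in range.
; A looping timer picks a target through the player, sphere-traces toward it, and ends the ability when no enemies remain.
; Each unique hit actor receives a set-by-caller damage effect using CalculateDamageWithArmor, and the player heals by a LifeSteal percentage of it.
; An invalid target triggers a next-tick retry, and debug trace drawing is on.
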(event `self.K2_OnEndAbility`
  (params (bWasCancelled :type Boolean))
  (`KismetSystemLibrary.K2_ClearAndInvalidateTimerHandle` (`self.HitScanTimer`))
  (set `/Game/Dynamic/Blueprints/Controllers/Player/BP_Player.IsAutoSwordAbilityActivated?` false (`self.PlayerRef`)))

(event `self.K2_ActivateAbility`
  (bind _output_get (set `self.PlayerRef` (cast `/Game/Dynamic/Blueprints/Controllers/Player/BP_Player` (`self.GetAvatarActorFromActorInfo`) :!pure true)))
  (if (not (`/Game/Dynamic/Blueprints/Controllers/Player/BP_Player.IsAutoSwordAbilityActivated?` _output_get))
    (set `/Game/Dynamic/Blueprints/Controllers/Player/BP_Player.IsAutoSwordAbilityActivated?` true _output_get)
    (bind _returnvalue (`KismetSystemLibrary.K2_SetTimerDelegate` (delegate `AutoSwordAttack`) 1.0 true false -1.0))
    (set `self.HitScanTimer` _returnvalue)
    (else
      (`self.K2_EndAbility`))))

(event `AutoSwordAttack`
  (bind _returnvalue (`self.GetAvatarActorFromActorInfo`))
  (bind _playerref (`self.PlayerRef`))
  (bind _returnvalue_2 (`AbilitySystemBlueprintLibrary.GetAbilitySystemComponent` (`self.GetAvatarActorFromActorInfo`)))
  (bind _returnvalue_3 (`Actor.K2_GetActorLocation` _returnvalue))
  (bind _enemiesinswordattackrange (`/Game/Dynamic/Blueprints/Controllers/Player/BP_Player.EnemiesInSwordAttackRange` _playerref))
  (bind _swordattackrange (`/Game/Dynamic/Blueprints/Controllers/Player/BP_Player.SwordAttackRange` _playerref))
  (bind (_lifesteal_basevalue _lifesteal_currentvalue) (break `GameplayAttributeData` (`BasicAttributeSet.LifeSteal` (`GASCharacterBase.BasicAttributeSet` (cast `GASCharacterBase` (`self.GetAvatarActorFromActorInfo`) :!pure true)))))
  (`KismetArrayLibrary.Array_Clear` (`self.HitActors`))
  (if (`KismetArrayLibrary.Array_IsNotEmpty` _enemiesinswordattackrange)
    (bind _attacktarget (message `/Game/Dynamic/Blueprints/GameplayAbilitySystem/Interfaces/BPI_Targetting.GetAttackTarget` _playerref _swordattackrange false _enemiesinswordattackrange _ :!label _label))
    (`/Engine/EditorBlueprintResources/StandardMacros.IsValid` _attacktarget
      (:`Is Valid`
        (bind _outhits (`KismetSystemLibrary.SphereTraceMultiForObjects` _returnvalue_3 (+ _returnvalue_3 (* (`KismetMathLibrary.Normal` (- (`Actor.K2_GetActorLocation` _attacktarget) _returnvalue_3)) (+ _swordattackrange 50.0))) 50.0 (`|MakeArray` "ObjectTypeQuery3" :!type "EObjectTypeQuery Enum") false (`|MakeArray` _returnvalue) "ForDuration" true (struct :`R` 1.0 :`B` 1.0 :`A` 1.0) (struct :`G` 1.0 :`A` 1.0) 0.066667))
        (`GameplayStatics.PlaySound2D` (`self.AttackSound`) 1.0 (`KismetMathLibrary.RandomFloatInRange` 0.9 1.1) 0.0 null null)
        (for _array_element _outhits
          (bind (_bblockinghit _binitialoverlap _time _distance _location _impactpoint _normal _impactnormal _physmat _hitactor _hitcomponent) (`GameplayStatics.BreakHitResult` _array_element))
          (bind _returnvalue_4 (`AbilitySystemBlueprintLibrary.GetAbilitySystemComponent` _hitactor))
          (`/Engine/EditorBlueprintResources/StandardMacros.IsValid` _returnvalue_4
            (:`Is Valid`
              (if (not (`KismetArrayLibrary.Array_Contains` (`self.HitActors`) _hitactor))
                (`KismetArrayLibrary.Array_AddUnique` (`self.HitActors`) _hitactor)
                (bind _damage (`self.CalculateDamageWithArmor` _hitactor))
                (bind _returnvalue_5 (`AbilitySystemBlueprintLibrary.AssignTagSetByCallerMagnitude` (`self.MakeOutgoingGameplayEffectSpec` "/Game/Dynamic/Blueprints/GameplayAbilitySystem/Effects/Damage/GE_Damage_Instant.GE_Damage_Instant_C") (struct :`TagName` "Data.Damage") _damage))
                (`AbilitySystemComponent.BP_ApplyGameplayEffectSpecToSelf` _returnvalue_4 _returnvalue_5)
                ; LifeSteal
                (bind _returnvalue_6 (`AbilitySystemBlueprintLibrary.AssignTagSetByCallerMagnitude` (`AbilitySystemComponent.MakeOutgoingSpec` :`self` _returnvalue_2 :`GameplayEffectClass` "/Game/Dynamic/Blueprints/LifeSteal/GE_RegenHealth.GE_RegenHealth_C") (struct :`TagName` "Regen.Health") (* _damage (/ _lifesteal_currentvalue 100.0) -1.0)))
                (`AbilitySystemComponent.BP_ApplyGameplayEffectSpecToSelf` _returnvalue_2 _returnvalue_6))))))
      (:`Is Not Valid`
        (`KismetSystemLibrary.DelayUntilNextTick`)
        (goto _label)))
    (else
      (`self.K2_EndAbility`))))