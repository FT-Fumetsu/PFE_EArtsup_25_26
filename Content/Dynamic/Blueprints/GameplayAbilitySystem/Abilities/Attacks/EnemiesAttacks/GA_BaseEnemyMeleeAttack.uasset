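; Base Gameplay Ability for enemy melee attacks that damages the player.
; On activation it sphere-traces from the avatar toward its target over its attack range, both fetched by message calls, ignoring every BP_Enemy_Base.
; A player hit applies GE_Damage_Instant with Damage as a SetByCaller magnitude.
; The ability ends only on that hit, and debug drawing and a "Hello" print remain.
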(event `self.K2_ActivateAbility`
  (`self.Attack`))

(event `self.K2_OnEndAbility`
  (params (bWasCancelled :type Boolean)))

(event `Attack`
  (bind _returnvalue (`self.GetAvatarActorFromActorInfo`))
  (bind _returnvalue_2 (`Actor.K2_GetActorLocation` _returnvalue))
  (bind _attacktarget (message `/Game/Dynamic/Blueprints/GameplayAbilitySystem/Interfaces/BPI_Targetting.GetAttackTarget` _returnvalue 0.0 false))
  (bind _attackrange (message `/Game/Dynamic/Blueprints/GameplayAbilitySystem/Interfaces/BPI_Targetting.GetAttackRange` _returnvalue))
  (bind _outactors (`GameplayStatics.GetAllActorsOfClass` "/Game/Dynamic/Blueprints/Controllers/Enemies/EnemyBase/BP_Enemy_Base.BP_Enemy_Base_C"))
  (bind _outhit (`KismetSystemLibrary.SphereTraceSingleForObjects` _returnvalue_2 (+ _returnvalue_2 (* (`KismetMathLibrary.Normal` (- (`Actor.K2_GetActorLocation` _attacktarget) _returnvalue_2)) _attackrange)) 50.0 (`|MakeArray` "ObjectTypeQuery3" :!type "EObjectTypeQuery Enum") false _outactors "ForDuration" true (struct :`B` 1.0 :`A` 1.0) (struct :`R` 1.0 :`B` 7.3e-05 :`A` 1.0) 0.066667))
  (`KismetSystemLibrary.PrintString` "Hello")
  (bind (_bblockinghit _binitialoverlap _time _distance _location _impactpoint _normal _impactnormal _physmat _hitactor) (`GameplayStatics.BreakHitResult` _outhit))
  (if (== _hitactor (`GameplayStatics.GetPlayerCharacter` 0))
    (bind _returnvalue_3 (`AbilitySystemBlueprintLibrary.AssignTagSetByCallerMagnitude` (`self.MakeOutgoingGameplayEffectSpec` "/Game/Dynamic/Blueprints/GameplayAbilitySystem/Effects/GE_Damage_Instant.GE_Damage_Instant_C") (struct :`TagName` "Data.Damage") (`self.Damage`)))
    (`AbilitySystemComponent.BP_ApplyGameplayEffectSpecToSelf` (`AbilitySystemBlueprintLibrary.GetAbilitySystemComponent` _hitactor) _returnvalue_3)
    (`self.K2_EndAbility`)))