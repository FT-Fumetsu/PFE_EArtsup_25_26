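; Base Gameplay Ability for enemy projectile attacks, firing at the avatar's attack target or, with none, straight ahead if HasPc passes, otherwise ending.
; ShootProjectile spawns a GAS projectile from the equipped weapon's spawn point, falling back to the actor's location.
; The projectile carries a damage effect spec set by caller magnitude, and a successful spawn ends the ability.
; The attack montage is disconnected and the ShootProjectile event wait triggers nothing.
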(event `self.K2_ActivateAbility`
  (`AbilityTask_WaitGameplayEvent.WaitGameplayEvent` (struct :`TagName` "Event.ShootProjectile") null
    (:`then`
      _)
    (:`EventReceived`
      _))
  (bind _attacktarget (message `/Game/Dynamic/Blueprints/GameplayAbilitySystem/Interfaces/BPI_Targetting.GetAttackTarget` (`self.GetAvatarActorFromActorInfo`) 0.0 false))
  (`/Engine/EditorBlueprintResources/StandardMacros.IsValid` _attacktarget
    (:`Is Valid`
      (`self.ShootProjectile` (`Actor.K2_GetActorLocation` _attacktarget)))
    (:`Is Not Valid`
      (if (`self.HasPc`)
        (`self.ShootProjectile` (+ (`self.SpawnLocation`) (* (`Actor.GetActorForwardVector` (`self.GetAvatarActorFromActorInfo`)) 10000.0)))
        (else
          (`self.K2_EndAbility`))))))

(event `ShootProjectile`
  (params (TargetLocation :type "Vector Structure"))
  (bind _returnvalue (`AbilitySystemBlueprintLibrary.AssignTagSetByCallerMagnitude` (`self.MakeOutgoingGameplayEffectSpec` (`self.Gameplay Effect Class`)) (struct :`TagName` "Data.Damage") (`self.DamageMagnitude`)))
  (bind _location (`self.GetSpawnLocation`))
  (bind _output_get (set `self.SpawnLocation` _location))
  (`GameplayTask_SpawnActor.SpawnActor` null _output_get (struct) "/Game/Dynamic/Blueprints/Attacks/Projectiles/BP_Projectile_GAS_Base_Child.BP_Projectile_GAS_Base_Child_C" false (`self.Speed`) TargetLocation _returnvalue (cast `Pawn` (`self.GetAvatarActorFromActorInfo`) :!pure true)
    (:`Success`
      (`self.K2_EndAbility`))
    (:`DidNotSpawn`
      (`KismetSystemLibrary.PrintString` "PROJECTILE NOT SPAWNED" true true (struct :`R` 1.0 :`A` 1.0)))))

(fn `GetSpawnLocation`
  (returns (Location :type "Vector Structure"))
  (bind _returnvalue (`self.GetAvatarActorFromActorInfo`))
  (bind _returnvalue_2 (`Actor.GetComponentByClass` _returnvalue "/Game/Dynamic/Blueprints/Weapons/AC_WeaponsManagerComponent.AC_WeaponsManagerComponent_C"))
  (`/Engine/EditorBlueprintResources/StandardMacros.IsValid` _returnvalue_2
    (:`Is Valid`
      (bind _equippedweapon (`/Game/Dynamic/Blueprints/Weapons/AC_WeaponsManagerComponent.EquippedWeapon` _returnvalue_2)
        (:`then`
          (bind _location (`/Game/Dynamic/Blueprints/Weapons/BP_Weapon_Base.GetSpawnPointLocation` _equippedweapon))
          (if (!= _location (0.0 0.0 0.0))
            (return _location)
            (else
              _)))
        (:`else`
          _)))
    (:`Is Not Valid`
      _))
  (return (`Actor.K2_GetActorLocation` _returnvalue)))