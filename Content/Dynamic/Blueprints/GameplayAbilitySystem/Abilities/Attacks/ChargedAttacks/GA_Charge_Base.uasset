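; Base gameplay ability for charged weapon attacks, apparently unfinished.
; On activation it commits, caches the equipped weapon from AC_WeaponsManagerComponent, loops AM_Attack_Loop and only prints when the GameplayAbility.ChargeRelease tag is added.
; Helper events bracket weapon hit scans with gameplay events, passing a SetByCaller damage spec with zero magnitude.
; The input-release charge loop and release montage that would trigger these helpers are disconnected.
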(event `LoopChargeAnimation`
  (`AbilityTask_PlayMontageAndWait.CreatePlayMontageAndWaitProxy` "None" (`self.ChargingMontage`) 1.0 "None" true 1.0 0.0 true
    (:`OnBlendOut`
      (if (`self.IsCharging?`)
        (`self.LoopChargeAnimation`)))
    (:`OnInterrupted`
      (if (`self.IsCharging?`)
        (`self.K2_EndAbility`)))))

(event `HandleHitScanStart`
  (bind _equipped_weapon (`self.Equipped Weapon`)
    (:`then`
      (bind _returnvalue (`AbilitySystemBlueprintLibrary.AssignTagSetByCallerMagnitude` (`self.MakeOutgoingGameplayEffectSpec` "/Game/Dynamic/Blueprints/GameplayAbilitySystem/Effects/GE_Damage_Instant.GE_Damage_Instant_C") (struct :`TagName` "Data.Damage")))
      (`/Game/Dynamic/Blueprints/Weapons/BP_Weapon_Base.HitScanStart` _equipped_weapon _returnvalue))
    (:`else`)))

(event `OnReleaseButton`
  (`AbilityTask_WaitGameplayEvent.WaitGameplayEvent` (struct :`TagName` "Event.HitScan.Start") null
    (:`then`
      (`AbilityTask_WaitGameplayEvent.WaitGameplayEvent` (struct :`TagName` "Event.HitScan.End") null
        (:`EventReceived`
          (`self.HandleHitScanEnd`))))
    (:`EventReceived`
      (`self.HandleHitScanStart`))))

(event `HandleHitScanEnd`
  (bind _equipped_weapon (`self.Equipped Weapon`)
    (:`then`
      (`/Game/Dynamic/Blueprints/Weapons/BP_Weapon_Base.HitScanEnd` _equipped_weapon))
    (:`else`)))

(event `self.K2_ActivateAbility`
  (bind _returnvalue (`Actor.GetComponentByClass` (`self.GetAvatarActorFromActorInfo`) "/Game/Dynamic/Blueprints/Weapons/AC_WeaponsManagerComponent.AC_WeaponsManagerComponent_C"))
  (`self.K2_CommitAbility`)
  (`/Engine/EditorBlueprintResources/StandardMacros.IsValid` _returnvalue
    (:`Is Valid`
      (bind _equippedweapon (`/Game/Dynamic/Blueprints/Weapons/AC_WeaponsManagerComponent.EquippedWeapon` _returnvalue)
        (:`then`
          (set `self.Equipped Weapon` _equippedweapon)
          (set `self.ChargeTime` 0.0)
          (`AbilityAsync_WaitGameplayTagAdded.WaitGameplayTagAddToActor` (`self.GetAvatarActorFromActorInfo`) (struct :`TagName` "GameplayAbility.ChargeRelease")
            (:`then`
              (`AbilityTask_PlayMontageAndWait.CreatePlayMontageAndWaitProxy` "None" "/Game/Static/DefaultUE5Characters/Mannequins/Anims/Unarmed/Attack/AM_Attack_Loop.AM_Attack_Loop" 1.0 "None" true 1.0 0.0 true :!label _label
                (:`OnBlendOut`
                  (goto _label))))
            (:`Added`
              (`KismetSystemLibrary.PrintString` "Release"))))
        (:`else`
          (`self.K2_EndAbility` :!label _label_2))))
    (:`Is Not Valid`
      (goto _label_2))))