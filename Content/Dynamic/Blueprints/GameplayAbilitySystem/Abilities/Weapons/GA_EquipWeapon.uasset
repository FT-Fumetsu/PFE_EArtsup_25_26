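; Gameplay ability that equips or unequips the avatar's weapon in response to a gameplay event.
; It commits, then switches on the event's first target tag to pick the gauntlets, sword or gun Blueprint class.
; The avatar's weapons manager component equips that class, or unequips on any other tag.
; The ability ends right after, but only when that component is valid, as the invalid path has no end call.
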(event `self.K2_ActivateAbilityFromEvent`
  (params (EventData :type "GameplayEventData Structure (by ref)"))
  (bind _returnvalue (`Actor.GetComponentByClass` (`self.GetAvatarActorFromActorInfo`) "/Game/Dynamic/Blueprints/Weapons/AC_WeaponsManagerComponent.AC_WeaponsManagerComponent_C"))
  (`self.K2_CommitAbility`)
  (`/Engine/EditorBlueprintResources/StandardMacros.IsValid` _returnvalue
    (:`Is Valid`
      (`|ExecutionSequence`
        (:`then_0`
          (`|SwitchGameplayTag` (`|GetArrayItem` (`BlueprintGameplayTagLibrary.BreakGameplayTagContainer` (`.TargetTags` (break `GameplayEventData` EventData))))
            (:`Default`
              (`/Game/Dynamic/Blueprints/Weapons/AC_WeaponsManagerComponent.UnequipWeapon` _returnvalue))
            (:`Weapon.Melee.Gauntelts`
              (`/Game/Dynamic/Blueprints/Weapons/AC_WeaponsManagerComponent.EquipWeapon` _returnvalue "/Game/Dynamic/Blueprints/Weapons/BP_Weapon_Gauntlets.BP_Weapon_Gauntlets_C"))
            (:`Weapon.MidRange.Sword`
              (`/Game/Dynamic/Blueprints/Weapons/AC_WeaponsManagerComponent.EquipWeapon` _returnvalue "/Game/Dynamic/Blueprints/Weapons/BP_Weapon_Sword.BP_Weapon_Sword_C"))
            (:`Weapon.Ranged.Gun`
              (`/Game/Dynamic/Blueprints/Weapons/AC_WeaponsManagerComponent.EquipWeapon` _returnvalue "/Game/Dynamic/Blueprints/Weapons/BP_Weapon_Gun.BP_Weapon_Gun_C"))))
        (:`then_1`
          (`self.K2_EndAbility`))))))