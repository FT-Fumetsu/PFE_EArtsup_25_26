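; Gameplay ability that scales an enemy's health, speed, damage and armor by the scaling level stored per enemy class in GS_Prototype.
; CalculateStats holds linear formulas over the enemy's FinalStats and EnemyScalingData.
; Activation passes magnitudes to GE_EnemyScalingStatistics via SetByCaller tags, adding armor only when the scale count equals its threshold.
; It retries each tick until scaling data is valid, then applies the effect and ends.
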(event `self.K2_ActivateAbility`
  (bind (_enemyscalingdata _healthmagnitude _speedmagnitude _attackmagnitude _armormagnitude) (`self.CalculateStats`))
  (set `self.NumberOfScales` (+ (`self.NumberOfScales`) 1))
  (set `self.ScaleLevel` (`BlueprintMapLibrary.Map_Find` (`/Game/Dynamic/Blueprints/Controllers/Player/GS_Prototype.ScalingLevelForClass` (cast `/Game/Dynamic/Blueprints/Controllers/Player/GS_Prototype` (`GameplayStatics.GetGameState`) :!pure true)) (`GameplayStatics.GetObjectClass` (cast `/Game/Dynamic/Blueprints/Controllers/Enemies/EnemyBase/BP_Enemy_Base` (`self.GetAvatarActorFromActorInfo`) :!pure true))))
  (`/Engine/EditorBlueprintResources/StandardMacros.IsValid` _enemyscalingdata :!label _label
    (:`Is Valid`
      (bind _returnvalue (`AbilitySystemBlueprintLibrary.AssignTagSetByCallerMagnitude` (`self.MakeOutgoingGameplayEffectSpec` "/Game/Dynamic/Blueprints/GameplayAbilitySystem/Effects/Stats/GE_EnemyScalingStatistics.GE_EnemyScalingStatistics_C") (struct :`TagName` "Enemy.Statistics.Scaling.MaxHealth") (`KismetMathLibrary.Conv_IntToDouble` _healthmagnitude)))
      (bind _returnvalue_2 (`AbilitySystemBlueprintLibrary.AssignTagSetByCallerMagnitude` _returnvalue (struct :`TagName` "Enemy.Statistics.Scaling.Speed") _speedmagnitude))
      (bind _returnvalue_3 (`AbilitySystemBlueprintLibrary.AssignTagSetByCallerMagnitude` _returnvalue_2 (struct :`TagName` "Enemy.Statistics.Scaling.Damage") _attackmagnitude))
      (set `self.SpecHandle` _returnvalue_3)
      (if (== (`self.NumberOfScales`) (`PDA_EnemyScaling.NumberOfLevelsToScaleArmor` _enemyscalingdata))
        (bind _returnvalue_4 (`AbilitySystemBlueprintLibrary.AssignTagSetByCallerMagnitude` _returnvalue_3 (struct :`TagName` "Enemy.Statistics.Scaling.Armor") _armormagnitude))
        (set `self.SpecHandle` _returnvalue_4))
      (`AbilitySystemComponent.BP_ApplyGameplayEffectSpecToSelf` (`AbilitySystemBlueprintLibrary.GetAbilitySystemComponent` (`self.GetAvatarActorFromActorInfo`)) (`self.SpecHandle`))
      (`self.K2_EndAbility`))
    (:`Is Not Valid`
      (`KismetSystemLibrary.DelayUntilNextTick`)
      (goto _label))))