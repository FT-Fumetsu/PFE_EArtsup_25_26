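; Base Gameplay Ability that automatically and repeatedly fires projectiles from the player on a cooldown.
; One-time activation binds to the player's new-target event and attempts a shot, either at an in-range enemy or along the avatar's forward vector when no target is needed.
; A delayed-loop macro spawns each volley from GetSpawnLocation, which returns the avatar's position.
; Successful spawns block shooting and set a cooldown timer that re-enables it and tries again.
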(event `self.K2_ActivateAbility`
  (`/Engine/EditorBlueprintResources/StandardMacros.DoOnce` false
    (:`Completed`
      (bind _output_get (set `self.PlayerRef` (cast `/Game/Dynamic/Blueprints/Controllers/Player/BP_Player` (`self.GetAvatarActorFromActorInfo`) :!pure true)))
      (add `/Game/Dynamic/Blueprints/Controllers/Player/BP_Player.OnNewTargetAquired` _output_get (`|CreateDelegate` :!event `TryShoot`))
      (`self.TryShoot`))))

(event `LoopSpawn`
  (bind _returnvalue (`KismetSystemLibrary.K2_SetTimerDelegate` (delegate `TimerSpawnProjectile`) (`self.Cooldown`) false true))
  (set `self.Timer` _returnvalue))

(event `TimerSpawnProjectile`
  (set `self.CanShoot?` true)
  (`self.TryShoot`))

(event `TryShoot`
  (bind _returnvalue (`self.GetAvatarActorFromActorInfo`))
  (if (`self.CanShoot?`)
    (bind _playerref (`self.PlayerRef`)
      (:`then`
        (if (`self.NeedsTarget?`)
          (bind _enemiesinprojectilerange (`/Game/Dynamic/Blueprints/Controllers/Player/BP_Player.EnemiesInProjectileRange` _playerref))
          (if (`KismetArrayLibrary.Array_IsNotEmpty` _enemiesinprojectilerange)
            (bind _projectilerange (message `/Game/Dynamic/Blueprints/GameplayAbilitySystem/Interfaces/BPI_Targetting.GetProjectileRange` _playerref))
            (bind _attacktarget (message `/Game/Dynamic/Blueprints/GameplayAbilitySystem/Interfaces/BPI_Targetting.GetAttackTarget` _playerref _projectilerange true _enemiesinprojectilerange _))
            (bind _output_get (set `self.Target` _attacktarget))
            (`/Engine/EditorBlueprintResources/StandardMacros.IsValid` _output_get :!label _label
              (:`Is Valid`
                (`self.ShootProjectile` (`Actor.K2_GetActorLocation` _output_get)))
              (:`Is Not Valid`
                (`KismetSystemLibrary.DelayUntilNextTick`)
                (goto _label))))
          (else
            (`self.ShootProjectile` (+ (* (`Actor.GetActorForwardVector` _returnvalue) (`self.NoTargetMultiplier`)) (`Actor.K2_GetActorLocation` _returnvalue))))))
      (:`else`))))

(event `ShootProjectile`
  (params (TargetLocation :type "Vector Structure"))
  (`self.ForLoopWithDelay` 0 (- (`self.NumberOfProjectiles`) 1) (`self.DelayBetweenProjectileSpawns`)
    (:`LoopBody`
      (bind _location (`self.GetSpawnLocation`))
      (bind _output_get (set `self.SpawnLocation` _location))
      (`GameplayTask_SpawnActor.SpawnActor` null _output_get (struct) (`self.ProjectileClass`) false TargetLocation (`self.Target`) (`self.Class to Ignore`) (cast `Pawn` (`self.GetAvatarActorFromActorInfo`) :!pure true)
        (:`Success`
          (set `self.CanShoot?` false)
          (`self.LoopSpawn`))
        (:`DidNotSpawn`
          (`KismetSystemLibrary.PrintString` "PLAYER PROJECTILE NOT SPAWNED" true true (struct :`R` 1.0 :`A` 1.0)))))))

(fn `GetSpawnLocation`
  (returns (Location :type "Vector Structure"))
  (return (`Actor.K2_GetActorLocation` (`self.GetAvatarActorFromActorInfo`))))