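; Gameplay ability that initializes a character's base stats through GAS when activated.
; It casts the avatar to BP_Player, or otherwise BP_Enemy_Base, and reads its DefaultStatsStruct.
; A helper builds a GE_DefaultCharacterStats spec, filling each stat via SetByCaller tags, with Health starting at MaxHealth.
; The spec is then applied to the avatar's own Ability System Component; EndAbility is never called.
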(event `self.K2_ActivateAbility`
  (bind _returnvalue (`self.GetAvatarActorFromActorInfo`))
  (bind _returnvalue_2 (`AbilitySystemBlueprintLibrary.GetAbilitySystemComponent` (`self.GetAvatarActorFromActorInfo`)))
  (bind _asbp_player (cast `/Game/Dynamic/Blueprints/Controllers/Player/BP_Player` _returnvalue)
    (:`then`
      (bind _spechandle (`self.ApplyGameplayEffectSpec` (`/Game/Dynamic/Blueprints/Controllers/Player/BP_Player.DefaultStatsStruct` _asbp_player)))
      (`AbilitySystemComponent.BP_ApplyGameplayEffectSpecToSelf` _returnvalue_2 _spechandle))
    (:`CastFailed`
      (bind _asbp_enemy_base (cast `/Game/Dynamic/Blueprints/Controllers/Enemies/EnemyBase/BP_Enemy_Base` _returnvalue))
      (bind _spechandle_2 (`self.ApplyGameplayEffectSpec` (`/Game/Dynamic/Blueprints/Controllers/Enemies/EnemyBase/BP_Enemy_Base.DefaultStatsStruct` _asbp_enemy_base)))
      (`AbilitySystemComponent.BP_ApplyGameplayEffectSpecToSelf` _returnvalue_2 _spechandle_2))))

(fn `ApplyGameplayEffectSpec`
  (params (DefaultStats :type "/Game/Dynamic/Blueprints/GameplayAbilitySystem/Effects/Stats/Str_DefaultStats Structure"))
  (returns (SpecHandle :type "GameplayEffectSpecHandle Structure"))
  (bind (_maxhealth _speed _lifesteal _armor _attackspeed _attack _dashdistance _dashtime _dashcooldown) (break `/Game/Dynamic/Blueprints/GameplayAbilitySystem/Effects/Stats/Str_DefaultStats` DefaultStats))
  (bind _returnvalue (`KismetMathLibrary.Conv_IntToDouble` _maxhealth))
  (bind _returnvalue_2 (`AbilitySystemBlueprintLibrary.AssignTagSetByCallerMagnitude` (`self.MakeOutgoingGameplayEffectSpec` "/Game/Dynamic/Blueprints/GameplayAbilitySystem/Effects/Stats/GE_DefaultCharacterStats.GE_DefaultCharacterStats_C") (struct :`TagName` "Statistics.Default.MaxHealth") _returnvalue))
  (bind _returnvalue_3 (`AbilitySystemBlueprintLibrary.AssignTagSetByCallerMagnitude` _returnvalue_2 (struct :`TagName` "Statistics.Default.Health") _returnvalue))
  (bind _returnvalue_4 (`AbilitySystemBlueprintLibrary.AssignTagSetByCallerMagnitude` _returnvalue_3 (struct :`TagName` "Statistics.Default.Speed") _speed))
  (bind _returnvalue_5 (`AbilitySystemBlueprintLibrary.AssignTagSetByCallerMagnitude` _returnvalue_4 (struct :`TagName` "Statistics.Default.LifeSteal") _lifesteal))
  (bind _returnvalue_6 (`AbilitySystemBlueprintLibrary.AssignTagSetByCallerMagnitude` _returnvalue_5 (struct :`TagName` "Statistics.Default.Armor") _armor))
  (bind _returnvalue_7 (`AbilitySystemBlueprintLibrary.AssignTagSetByCallerMagnitude` _returnvalue_6 (struct :`TagName` "Statistics.Default.AttackSpeed") _attackspeed))
  (bind _returnvalue_8 (`AbilitySystemBlueprintLibrary.AssignTagSetByCallerMagnitude` _returnvalue_7 (struct :`TagName` "Statistics.Default.Attack") _attack))
  (bind _returnvalue_9 (`AbilitySystemBlueprintLibrary.AssignTagSetByCallerMagnitude` _returnvalue_8 (struct :`TagName` "Statistics.Default.DashDistance") _dashdistance))
  (bind _returnvalue_10 (`AbilitySystemBlueprintLibrary.AssignTagSetByCallerMagnitude` _returnvalue_9 (struct :`TagName` "Statistics.Default.DashTime") _dashtime))
  (bind _returnvalue_11 (`AbilitySystemBlueprintLibrary.AssignTagSetByCallerMagnitude` _returnvalue_10 (struct :`TagName` "Statistics.Default.DashCooldown") _dashcooldown))
  (return _returnvalue_11))