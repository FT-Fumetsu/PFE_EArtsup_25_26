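; BP_EquipProjectiles is an interactable effect actor that gives the player a gameplay ability, by its name one that equips projectiles.
; Sphere overlap caches the BP_Player and shows a WBP_PressF prompt, created at BeginPlay and removed when that player leaves.
; Interact grants AbilityToGrant to the cached player's Ability System Component, then immediately activates it by class.
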(event `self.ReceiveBeginPlay`
  (bind _returnvalue (`|CreateWidget` "/Game/Dynamic/Blueprints/WidgetBlueprint(WBP)/Prototype/WBP_PressF.WBP_PressF_C"))
  (set `self.Widget` _returnvalue))

(event `/Game/Dynamic/Blueprints/InteractibleSystem/Interfaces/BPI_Interaction.Interact`
  (bind _abilitytogrant (`self.AbilityToGrant`))
  (bind _returnvalue (`AbilitySystemBlueprintLibrary.GetAbilitySystemComponent` (`self.PlayerRef`)))
  (`AbilitySystemComponent.K2_GiveAbility` _returnvalue _abilitytogrant 0 -1)
  (`AbilitySystemComponent.TryActivateAbilityByClass` _returnvalue _abilitytogrant true))

(event `self.Sphere.OnComponentBeginOverlap`
  (params (OverlappedComponent :type "PrimitiveComponent Object Reference") (OtherActor :type "Actor Object Reference") (OtherComp :type "PrimitiveComponent Object Reference") (OtherBodyIndex :type Integer) (bFromSweep :type Boolean) (SweepResult :type "HitResult Structure (by ref)"))
  (bind _asbp_player (cast `/Game/Dynamic/Blueprints/Controllers/Player/BP_Player` OtherActor))
  (set `self.PlayerRef` _asbp_player)
  (`UserWidget.AddToViewport` (`self.Widget`) 0))

(event `self.Sphere.OnComponentEndOverlap`
  (params (OverlappedComponent :type "PrimitiveComponent Object Reference") (OtherActor :type "Actor Object Reference") (OtherComp :type "PrimitiveComponent Object Reference") (OtherBodyIndex :type Integer))
  (if (== OtherActor (`self.PlayerRef`))
    (`Widget.RemoveFromParent` (`self.Widget`))))

(fn `UserConstructionScript`)