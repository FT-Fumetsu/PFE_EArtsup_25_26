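; Base area-of-effect actor that applies a GameplayEffect to overlapping actors with an Ability System Component, excluding its instigator.
; On entry, it skips targets already owning the magnitude tag, tracks the others, and applies the effect using that tag as the SetByCaller key.
; Leaving the area or destroying the actor removes all stacks of the effect class.
; A positive LifeTime makes it self-destroy through Tick.
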(event `self.ReceiveTick`
  (params (DeltaSeconds :type "Float (single-precision)"))
  (if (> (`self.LifeTime`) 0.0)
    (bind _output_get (set `self.ElapsedTime` (+ DeltaSeconds (`self.ElapsedTime`))))
    (if (>= _output_get (`self.LifeTime`))
      (`self.K2_DestroyActor`))))

(event `self.ReceiveActorBeginOverlap`
  (params (OtherActor :type "Actor Object Reference"))
  (bind _returnvalue (`AbilitySystemBlueprintLibrary.GetAbilitySystemComponent` OtherActor))
  (if (not (== OtherActor (`self.GetInstigator`)))
    (`/Engine/EditorBlueprintResources/StandardMacros.IsValid` _returnvalue
      (:`Is Valid`
        (if (not (`GameplayTagAssetInterface.HasMatchingGameplayTag` _returnvalue (`self.EffectMagnitudeDataType`)))
          (`KismetArrayLibrary.Array_AddUnique` (`self.ActorsInArea`) OtherActor)
          (bind _returnvalue_2 (`AbilitySystemBlueprintLibrary.MakeSpecHandleByClass` (`self.EffectClass`) null self))
          (bind _returnvalue_3 (`AbilitySystemBlueprintLibrary.AssignTagSetByCallerMagnitude` _returnvalue_2 (`self.EffectMagnitudeDataType`) (`self.EffectMagnitudeValue`)))
          (`AbilitySystemComponent.BP_ApplyGameplayEffectSpecToSelf` _returnvalue _returnvalue_3))))))

(event `self.ReceiveActorEndOverlap`
  (params (OtherActor :type "Actor Object Reference"))
  (bind _returnvalue (`AbilitySystemBlueprintLibrary.GetAbilitySystemComponent` OtherActor))
  (`/Engine/EditorBlueprintResources/StandardMacros.IsValid` _returnvalue
    (:`Is Valid`
      (`KismetArrayLibrary.Array_RemoveItem` (`self.ActorsInArea`) OtherActor)
      (`AbilitySystemComponent.RemoveActiveGameplayEffectBySourceEffect` _returnvalue (`self.EffectClass`) null -1)
      (`AbilitySystemComponent.GetActiveEffectsWithAllTags` _returnvalue (`BlueprintGameplayTagLibrary.MakeGameplayTagContainerFromTag` (`self.EffectMagnitudeDataType`))))))

(event `self.ReceiveDestroyed`
  (for _array_element (`self.ActorsInArea`)
    (bind _returnvalue (`AbilitySystemBlueprintLibrary.GetAbilitySystemComponent` _array_element))
    (`/Engine/EditorBlueprintResources/StandardMacros.IsValid` _returnvalue
      (:`Is Valid`
        (`AbilitySystemComponent.RemoveActiveGameplayEffectBySourceEffect` _returnvalue (`self.EffectClass`) null -1)))))

(fn `UserConstructionScript`)