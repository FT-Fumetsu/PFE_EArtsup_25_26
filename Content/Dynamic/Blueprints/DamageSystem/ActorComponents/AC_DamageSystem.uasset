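; AC_DamageSystem is an actor component that manages an actor's health, healing, damage and death.
; TakeDamage reads a damage info struct and uses a CanBeDamaged check to block, apply or ignore the hit, based on death, invincibility and blocking.
; Dispatchers report blocks with a parry flag, deaths, and damage responses when interruptible or forced.
; Healing clamps to max health and is skipped when dead.
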(fn `Heal`
  (params (Amount :type "Float (double-precision)"))
  (returns (NewHealth :type "Float (double-precision)"))
  (if (not (`self.IsDead?`))
    (bind _output_get (set `self.Health` (`KismetMathLibrary.FClamp` (+ Amount (`self.Health`)) 0.0 (`self.MaxHealth`))))
    (return _output_get)))

(fn `TakeDamage`
  (params (DamageInfos :type "/Game/Dynamic/Blueprints/DamageSystem/Structures/Str_DamageInfo Structure"))
  (returns (`WasDamaged?` :type Boolean))
  (bind (_amount _damagetype _damageresponse _shoulddamageinvincible_ _canbeblocked_ _canbeparried_ _shouldforceinterupt_) (break `/Game/Dynamic/Blueprints/DamageSystem/Structures/Str_DamageInfo` DamageInfos))
  (`self.CanBeDamaged?` _shoulddamageinvincible_ _canbeblocked_
    (:`BlockDame`
      (`self.OnBlocked` _canbeparried_)
      (return false))
    (:`DoDamege`
      (bind _output_get (set `self.Health` (- (`self.Health`) _amount)))
      (if (<= _output_get 0.0)
        (set `self.IsDead?` true)
        (`self.OnDeath`)
        (return true)
        (elif (or (`self.IsIterruptible?`) _shouldforceinterupt_)
          (`self.OnDamageResponse` _damageresponse)
          (return true))))
    (:`NoDamage`
      (return false))))