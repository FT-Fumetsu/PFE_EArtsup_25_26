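; XP coin pickup that homes in on the player and grants a Gameplay Effect on contact.
; MagnetArea, sized at BeginPlay, toggles magnetization for player pawn 0; Tick then interpolates the coin toward it, faster as distance shrinks, up to MaxSpeed.
; DestroyArea applies the effect with a SetByCaller magnitude to any overlapping actor with an Ability System Component, but destroys the coin only for BP_Player.
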(event `self.ReceiveBeginPlay`
  (`SphereComponent.SetSphereRadius` (`self.MagnetArea`) (`self.MagnetAreaRadius`) true))

(event `self.DestroyArea.OnComponentBeginOverlap`
  (params (OverlappedComponent :type "PrimitiveComponent Object Reference") (OtherActor :type "Actor Object Reference") (OtherComp :type "PrimitiveComponent Object Reference") (OtherBodyIndex :type Integer) (bFromSweep :type Boolean) (SweepResult :type "HitResult Structure (by ref)"))
  (bind _returnvalue (`AbilitySystemBlueprintLibrary.GetAbilitySystemComponent` OtherActor))
  (`/Engine/EditorBlueprintResources/StandardMacros.IsValid` _returnvalue
    (:`Is Valid`
      (bind _returnvalue_2 (`AbilitySystemBlueprintLibrary.MakeSpecHandleByClass` (`self.EffectClass`) null self))
      (bind _returnvalue_3 (`AbilitySystemBlueprintLibrary.AssignTagSetByCallerMagnitude` _returnvalue_2 (`self.EffectMagnitudeDataType`) (`self.EffectMagnitudeValue`)))
      (`AbilitySystemComponent.BP_ApplyGameplayEffectSpecToSelf` _returnvalue _returnvalue_3)
      (bind _asbp_player (cast `/Game/Dynamic/Blueprints/Controllers/Player/BP_Player` OtherActor))
      (`self.K2_DestroyActor`))))

(event `self.MagnetArea.OnComponentBeginOverlap`
  (params (OverlappedComponent :type "PrimitiveComponent Object Reference") (OtherActor :type "Actor Object Reference") (OtherComp :type "PrimitiveComponent Object Reference") (OtherBodyIndex :type Integer) (bFromSweep :type Boolean) (SweepResult :type "HitResult Structure (by ref)"))
  (if (== OtherActor (`GameplayStatics.GetPlayerPawn` 0))
    (set `self.IsMagnetized` true)))

(event `self.MagnetArea.OnComponentEndOverlap`
  (params (OverlappedComponent :type "PrimitiveComponent Object Reference") (OtherActor :type "Actor Object Reference") (OtherComp :type "PrimitiveComponent Object Reference") (OtherBodyIndex :type Integer))
  (if (== OtherActor (`GameplayStatics.GetPlayerPawn` 0))
    (set `self.IsMagnetized` false)))

(event `self.ReceiveTick`
  (params (DeltaSeconds :type "Float (single-precision)"))
  (bind _returnvalue (- (`self.K2_GetActorLocation` (`GameplayStatics.GetPlayerPawn` 0)) (`self.K2_GetActorLocation`)))
  (if (`self.IsMagnetized`)
    (set `self.Distance` (`KismetMathLibrary.VSize` _returnvalue))
    (set `self.Direction` (`KismetMathLibrary.Normal` _returnvalue))
    (bind _output_get (set `self.Speed` (`KismetMathLibrary.FClamp` (/ (`self.MagnetAreaRadius`) (`self.Distance`)) 0.0 (`self.MaxSpeed`))))
    (`self.K2_SetActorLocation` (`KismetMathLibrary.VInterpTo` (`self.K2_GetActorLocation`) (`self.K2_GetActorLocation` (`GameplayStatics.GetPlayerPawn` 0)) DeltaSeconds _output_get))))

(fn `UserConstructionScript`)