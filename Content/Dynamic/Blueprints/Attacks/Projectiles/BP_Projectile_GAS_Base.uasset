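; Base projectile for GAS attacks that flies toward a target location, plays random spawn and destroy sounds, and expires after its lifetime.
; The overlap event is empty, with helper functions provided for hit filtering and environment collision cleanup.
; Valid hits apply an armor-reduced SetByCaller damage effect to the target and a LifeSteal-scaled heal to the instigator.
; Environment hits destroy the overlapped component and its children, or the actor if none is valid.
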(event `self.ReceiveTick`
  (params (DeltaSeconds :type "Float (single-precision)"))
  (bind _output_get (set `self.ElapsedTime` (+ DeltaSeconds (`self.ElapsedTime`))))
  (if (and (>= _output_get (`self.LifeTime`)) (> (`self.LifeTime`) 0.0))
    (`self.K2_DestroyActor`)))

(event `self.ReceiveBeginPlay`
  (bind _projectilemovement (`self.ProjectileMovement`))
  (set `MovementComponent.Velocity` (* (`KismetMathLibrary.GetDirectionUnitVector` (`self.K2_GetActorLocation`) (`self.TargetLocation`)) (`self.Speed`)) _projectilemovement)
  (`ActorComponent.Activate` _projectilemovement false)
  (`PrimitiveComponent.IgnoreActorWhenMoving` (`self.SphereCollider`) (`self.GetInstigator`) false)
  (`GameplayStatics.SpawnSoundAtLocation` (`KismetArrayLibrary.Array_Random` (`self.SpawnSound`)) (`self.K2_GetActorLocation`) (struct) (`self.VolumeMultiplier`) (`KismetMathLibrary.RandomFloatInRange` 0.8 1.2) 0.0 "/Game/Static/07_SFX/SFX/ATT_Projectiles.ATT_Projectiles" "/Game/Static/07_SFX/SFX/SC_ProjectilesConcurrencySettings.SC_ProjectilesConcurrencySettings"))

(event `self.SphereCollider.OnComponentBeginOverlap`
  (params (OverlappedComponent :type "PrimitiveComponent Object Reference") (OtherActor :type "Actor Object Reference") (OtherComp :type "PrimitiveComponent Object Reference") (OtherBodyIndex :type Integer) (bFromSweep :type Boolean) (SweepResult :type "HitResult Structure (by ref)")))

(event `self.ReceiveDestroyed`
  (`self.OnDestroyedComponent`))

(event `OnDestroyedComponent`
  (`GameplayStatics.SpawnSoundAtLocation` (`KismetArrayLibrary.Array_Random` (`self.DestroyedSound`)) (`self.K2_GetActorLocation`) (struct) (`self.VolumeMultiplier`) (`KismetMathLibrary.RandomFloatInRange` 0.8 1.2) 0.0 "/Game/Static/07_SFX/SFX/ATT_Projectiles.ATT_Projectiles" "/Game/Static/07_SFX/SFX/SC_ProjectilesConcurrencySettings.SC_ProjectilesConcurrencySettings"))

(fn `CheckIfEnvironmentOverlapped`
  (params (OtherComponent :type "PrimitiveComponent Object Reference"))
  (returns (Environment :type Boolean))
  (switch `ECollisionChannel` (`PrimitiveComponent.GetCollisionObjectType` OtherComponent)
    (:`ECC_WorldStatic`
      _)
    (:`ECC_WorldDynamic`
      _)
    (:`ECC_Pawn`
      (return false))
    (:`ECC_Visibility`
      (return false))
    (:`ECC_Camera`
      (return false))
    (:`ECC_PhysicsBody`
      (return false))
    (:`ECC_Vehicle`
      (return false))
    (:`ECC_Destructible`
      (return false))
    (:`ECC_GameTraceChannel1`
      (return false))
    (:`ECC_GameTraceChannel2`
      (return false))
    (:`ECC_GameTraceChannel3`
      _)
    (:`ECC_GameTraceChannel4`
      (return false))
    (:`ECC_GameTraceChannel5`
      (return false)))
  (return true))

(fn `CheckOverlappedActorIsEnemy`
  (params (OtherActor :type "Actor Object Reference") (DamageValue :type "Float (double-precision)"))
  (returns (Success :type Boolean))
  (locals (NewLocalVar :type "GameplayEffect Class Reference"))
  (bind _returnvalue (`AbilitySystemBlueprintLibrary.GetAbilitySystemComponent` OtherActor))
  (castclass `/Game/Dynamic/Blueprints/Controllers/Enemies/EnemyBase/BP_Enemy_Base` (`GameplayStatics.GetObjectClass` OtherActor)
    (:`then`
      (if (!= "/Game/Dynamic/Blueprints/Controllers/Enemies/EnemyBase/BP_Enemy_Base.BP_Enemy_Base_C" (`self.ClassToIgnore`))
        (if (!= OtherActor (`self.Instigator`)) :!label _label
          (`/Engine/EditorBlueprintResources/StandardMacros.IsValid` _returnvalue
            (:`Is Valid`
              (`self.MakeGameplayEffectSpec` OtherActor DamageValue)
              (set `self.OverlappedActorASC` _returnvalue)
              (return true)))
          (else
            _))))
    (:`CastFailed`
      (goto _label)))
  (return false))

(fn `MakeGameplayEffectSpec`
  (params (OtherActor :type "Actor Object Reference") (DamageMagnitude :type "Float (double-precision)"))
  (bind _returnvalue (`AbilitySystemBlueprintLibrary.GetAbilitySystemComponent` OtherActor))
  (bind _returnvalue_2 (`AbilitySystemBlueprintLibrary.GetAbilitySystemComponent` (`self.GetInstigator`)))
  (bind (_armor_basevalue _armor_currentvalue) (break `GameplayAttributeData` (`BasicAttributeSet.Armor` (`GASCharacterBase.BasicAttributeSet` (cast `GASCharacterBase` OtherActor :!pure true)))))
  (bind (_lifesteal_basevalue _lifesteal_currentvalue) (break `GameplayAttributeData` (`BasicAttributeSet.LifeSteal` (`GASCharacterBase.BasicAttributeSet` (cast `GASCharacterBase` (`self.GetInstigator`) :!pure true)))))
  (bind _returnvalue_3 (`KismetMathLibrary.FClamp` (+ _armor_currentvalue DamageMagnitude) -10000.0 -1.0))
  (bind _returnvalue_4 (`AbilitySystemBlueprintLibrary.AssignTagSetByCallerMagnitude` (`AbilitySystemComponent.MakeOutgoingSpec` :`self` _returnvalue :`GameplayEffectClass` (`self.GameplayEffectClass`)) (`self.GameplayEffectDataTag`) _returnvalue_3))
  (`AbilitySystemComponent.BP_ApplyGameplayEffectSpecToSelf` _returnvalue _returnvalue_4)
  (bind _returnvalue_5 (`AbilitySystemBlueprintLibrary.AssignTagSetByCallerMagnitude` (`AbilitySystemComponent.MakeOutgoingSpec` :`self` _returnvalue_2 :`GameplayEffectClass` "/Game/Dynamic/Blueprints/LifeSteal/GE_RegenHealth.GE_RegenHealth_C") (struct :`TagName` "Regen.Health") (* _returnvalue_3 (/ _lifesteal_currentvalue 100.0) -1.0)))
  (`AbilitySystemComponent.BP_ApplyGameplayEffectSpecToSelf` _returnvalue_2 _returnvalue_5))

(fn `OnProjectileOverlap`
  (params (OverlapedComponent :type "PrimitiveComponent Object Reference") (OtherComponent :type "PrimitiveComponent Object Reference"))
  (bind _environment (`self.CheckIfEnvironmentOverlapped` OtherComponent))
  (if _environment
    (`/Engine/EditorBlueprintResources/StandardMacros.IsValid` OverlapedComponent
      (:`Is Valid`
        (for _array_element (`SceneComponent.GetChildrenComponents` OverlapedComponent true)
          (`ActorComponent.K2_DestroyComponent` _array_element))
        (`ActorComponent.K2_DestroyComponent` OverlapedComponent))
      (:`Is Not Valid`
        (`self.K2_DestroyActor`)))))

(fn `UserConstructionScript`)