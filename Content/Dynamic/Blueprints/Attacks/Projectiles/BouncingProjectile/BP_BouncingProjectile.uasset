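; Player projectile that bounces from enemy to enemy, applying its Damage value through an enemy overlap check.
; Each valid hit resets elapsed time, updates the ignore list (cleared first if same-actor bouncing is allowed) and destroys the projectile once its bounce limit is exceeded.
; Otherwise it asks the instigator for a new target among the player's in-range enemies and redirects its movement velocity toward it.
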(event `self.ReceiveBeginPlay`
  (`parent.ReceiveBeginPlay`))

(event `self.SphereCollider.OnComponentBeginOverlap`
  (params (OverlappedComponent :type "PrimitiveComponent Object Reference") (OtherActor :type "Actor Object Reference") (OtherComp :type "PrimitiveComponent Object Reference") (OtherBodyIndex :type Integer) (bFromSweep :type Boolean) (SweepResult :type "HitResult Structure (by ref)"))
  (bind _returnvalue (`self.GetInstigator`))
  (set `self.ElapsedTime` 0.0)
  (set `self.IsIgnoreActor` false)
  (for _array_element (`self.ActorsToIgnore`)
    (if (== OtherActor _array_element)
      (set `self.IsIgnoreActor` true)
      (break)))
  (if (not (`self.IsIgnoreActor`))
    (bind _success (`self.CheckOverlappedActorIsEnemy` OtherActor (`self.Damage`)))
    (if _success
      (if (`self.CanBounceOnSameActor?`)
        (`KismetArrayLibrary.Array_Clear` (`self.ActorsToIgnore`)))
      (`KismetArrayLibrary.Array_AddUnique` (`self.ActorsToIgnore`))
      (bind _output_get (set `self.CurrentBouncingNumber` (+ (`self.CurrentBouncingNumber`) 1)))
      (if (> _output_get (`self.BouncingNumber`))
        (`self.K2_DestroyActor`)
        (else
          (`PrimitiveComponent.IgnoreActorWhenMoving` (`self.SphereCollider`) OtherActor true)
          (bind _projectilerange (message `/Game/Dynamic/Blueprints/GameplayAbilitySystem/Interfaces/BPI_Targetting.GetProjectileRange` _returnvalue))
          (bind _attacktarget (message `/Game/Dynamic/Blueprints/GameplayAbilitySystem/Interfaces/BPI_Targetting.GetAttackTarget` _returnvalue _projectilerange true (`/Game/Dynamic/Blueprints/Controllers/Player/BP_Player.EnemiesInProjectileRange` (cast `/Game/Dynamic/Blueprints/Controllers/Player/BP_Player` _returnvalue :!pure true)) (`self.ActorsToIgnore`)))
          (`/Engine/EditorBlueprintResources/StandardMacros.IsValid` _attacktarget
            (:`Is Valid`
              (set `MovementComponent.Velocity` (* (`KismetMathLibrary.GetDirectionUnitVector` (`self.K2_GetActorLocation`) (`self.K2_GetActorLocation` _attacktarget)) (`self.Speed`)) (`self.ProjectileMovement`)))
            (:`Is Not Valid`
              (`KismetSystemLibrary.PrintString` "Bouncing Projectile : Attack Target not valid !!"))))))))

(fn `UserConstructionScript`
  (`parent.UserConstructionScript`))