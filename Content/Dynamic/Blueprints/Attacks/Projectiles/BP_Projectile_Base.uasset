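; Base projectile actor for attacks, moved by a projectile movement component configured from exposed speed and gravity settings in the construction script.
; On spawn it ignores collision with its owner and destroys itself after its lifetime unless flagged infinite.
; A box collider hit calls the OnProjectileImpact dispatcher, plays optional impact particles and sound at the hit location, then destroys the projectile.
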(event `self.ReceiveBeginPlay`
  (`|ExecutionSequence`
    (:`then_0`
      (`PrimitiveComponent.IgnoreActorWhenMoving` (`self.BoxCollider`) (`self.GetOwner`) true))
    (:`then_1`
      (if (not (`self.Infinite?`))
        (`KismetSystemLibrary.Delay` (`self.LifeTime`))
        (`self.K2_DestroyActor`)))))

(event `self.BoxCollider.OnComponentHit`
  (params (HitComponent :type "PrimitiveComponent Object Reference") (OtherActor :type "Actor Object Reference") (OtherComp :type "PrimitiveComponent Object Reference") (NormalImpulse :type "Vector Structure") (Hit :type "HitResult Structure (by ref)"))
  (bind (_bblockinghit _binitialoverlap _time _distance _location) (`GameplayStatics.BreakHitResult` Hit))
  (`self.OnProjectileImpact` OtherActor Hit)
  (bind _impacteffect (`self.ImpactEffect`)
    (:`then`
      (`GameplayStatics.SpawnEmitterAtLocation` _impacteffect _location))
    (:`else`
      _))
  (bind _impactsound (`self.ImpactSound`)
    (:`then`
      (`GameplayStatics.PlaySoundAtLocation` _impactsound _location (struct) 1.0 1.0 0.0 null null null null))
    (:`else`
      _))
  (`self.K2_DestroyActor`))

(fn `UserConstructionScript`
  (bind _projectilemovement (`self.ProjectileMovement`))
  (set `ProjectileMovementComponent.InitialSpeed` (`self.Speed`) _projectilemovement)
  (set `ProjectileMovementComponent.MaxSpeed` (`self.MaxSpeed`) _projectilemovement)
  (set `ProjectileMovementComponent.ProjectileGravityScale` (`self.GravityScale`) _projectilemovement))