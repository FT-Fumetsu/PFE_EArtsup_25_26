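; Base projectile Blueprint for attacks that home in on one specific Target actor.
; The construction script applies the homing acceleration and sets the target's root component as the ProjectileMovement homing target, destroying the projectile if Target is invalid.
; On BeginPlay, RotateToTarget points the initial velocity straight at the target at Speed, leaving ProjectileMovement's built-in homing to steer it.
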(event `self.ReceiveBeginPlay`
  (`parent.ReceiveBeginPlay`)
  (`self.Target`
    (:`then`
      (`self.RotateToTarget`))
    (:`else`)))

(event `RotateToTarget`
  (set `MovementComponent.Velocity` (* (`KismetMathLibrary.GetDirectionUnitVector` (`self.K2_GetActorLocation`) (`self.K2_GetActorLocation` (`self.Target`))) (`self.Speed`)) (`self.ProjectileMovement`)))

(fn `UserConstructionScript`
  (bind _projectilemovement (`self.ProjectileMovement`))
  (`parent.UserConstructionScript`)
  (set `ProjectileMovementComponent.HomingAccelerationMagnitude` (`self.HomingAcceleration`) _projectilemovement)
  (bind _target (`self.Target`)
    (:`then`
      (set `ProjectileMovementComponent.HomingTargetComponent` (`Actor.RootComponent` _target) _projectilemovement)
      (set `ProjectileMovementComponent.bIsHomingProjectile` true _projectilemovement))
    (:`else`
      (`self.K2_DestroyActor`))))