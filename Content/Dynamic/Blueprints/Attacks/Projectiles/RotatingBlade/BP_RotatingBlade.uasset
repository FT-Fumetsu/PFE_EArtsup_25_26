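; Rotating blade attack projectile that flies until it hits an enemy or a set delay passes, then stops and spins in place.
; On switching, it zeroes velocity once, spawns an infinite damage-over-time effect area at its position and spins the VFX with a timeline.
; When a positive lifetime expires, it destroys both the damage area and itself.
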(event `self.ReceiveBeginPlay`
  (`parent.ReceiveBeginPlay`)
  (set `self.IsRotating` false))

(event `self.ReceiveTick`
  (params (DeltaSeconds :type "Float (single-precision)"))
  (bind _output_get (set `self.ElapsedTime` (+ DeltaSeconds (`self.ElapsedTime`))))
  (if (and (>= _output_get (`self.LifeTime`)) (> (`self.LifeTime`) 0.0))
    (`self.K2_DestroyActor` (`self.DamageActor`))
    (`self.K2_DestroyActor`)
    (elif (`self.IsRotating`)
      (`/Engine/EditorBlueprintResources/StandardMacros.DoOnce` false
        (:`Completed`
          (set `MovementComponent.Velocity` (0.0 0.0 0.0) (`self.ProjectileMovement`))
          (bind _returnvalue (`|SpawnActorFromClass` "/Game/Dynamic/Blueprints/GameplayAbilitySystem/EffectActors/BP_EffectArea_Damage.BP_EffectArea_Damage_C" (`self.GetTransform`) "Undefined" "MultiplyWithRoot" null "/Game/Dynamic/Blueprints/GameplayAbilitySystem/Effects/Damage/GE_DamageOverTime_Infinite.GE_DamageOverTime_Infinite_C" (struct :`TagName` "Data.Damage") (`self.DamageInRotatingMode`) 0.0 null))
          (set `self.DamageActor` _returnvalue)
          (bind (_direction _rotate) (`Timeline|RotateBlade` :!via `PlayFromStart`)
            (:`Update`
              (`SceneComponent.K2_SetWorldRotation` (`self.VFX`) (`KismetMathLibrary.RLerp` (struct) (struct :`Yaw` 360.0) _rotate) false false)))))
      (elif (>= (`self.ElapsedTime`) (`self.TimeBeforeRotating`))
        (set `self.IsRotating` true)))))

(event `self.SphereCollider.OnComponentBeginOverlap`
  (params (OverlappedComponent :type "PrimitiveComponent Object Reference") (OtherActor :type "Actor Object Reference") (OtherComp :type "PrimitiveComponent Object Reference") (OtherBodyIndex :type Integer) (bFromSweep :type Boolean) (SweepResult :type "HitResult Structure (by ref)"))
  (if (not (`self.IsRotating`))
    (bind _success (`self.CheckOverlappedActorIsEnemy` OtherActor (`self.Damage`)))
    (if _success
      (set `self.IsRotating` true))))

(fn `UserConstructionScript`
  (`parent.UserConstructionScript`))