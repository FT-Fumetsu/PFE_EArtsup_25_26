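; Boomerang projectile attack that flies out, then homes back to the actor that fired it.
; After a set time, or on hitting an enemy with damage, it switches to returning and steers its velocity toward the instigator each tick.
; It is destroyed on overlapping the instigator, whose collision is briefly ignored at spawn so it can launch cleanly.
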(event `self.ReceiveBeginPlay`
  (`parent.ReceiveBeginPlay`)
  (`PrimitiveComponent.IgnoreActorWhenMoving` (`self.SphereCollider`) (`self.GetInstigator`) true)
  (`PrimitiveComponent.IgnoreActorWhenMoving` (`Character.CapsuleComponent` (`GameplayStatics.GetPlayerCharacter` 0)) self true)
  (`KismetSystemLibrary.Delay` 0.1)
  (`PrimitiveComponent.IgnoreActorWhenMoving` (`self.SphereCollider`) (`self.GetInstigator`) false))

(event `self.ReceiveTick`
  (params (DeltaSeconds :type "Float (single-precision)"))
  (`parent.ReceiveTick` DeltaSeconds)
  (if (`self.IsReturning`)
    (set `MovementComponent.Velocity` (* (`KismetMathLibrary.GetDirectionUnitVector` (`self.K2_GetActorLocation`) (`self.K2_GetActorLocation` (`self.GetInstigator`))) (`self.ReturnSpeed`)) (`self.ProjectileMovement`))
    (elif (>= (`self.ElapsedTime`) (`self.TimeBeforeReturning`))
      (set `self.IsReturning` true))))

(event `self.SphereCollider.OnComponentBeginOverlap`
  (params (OverlappedComponent :type "PrimitiveComponent Object Reference") (OtherActor :type "Actor Object Reference") (OtherComp :type "PrimitiveComponent Object Reference") (OtherBodyIndex :type Integer) (bFromSweep :type Boolean) (SweepResult :type "HitResult Structure (by ref)"))
  (`self.OnProjectileOverlap` null OtherComp)
  (bind _success (`self.CheckOverlappedActorIsEnemy` OtherActor (`self.Damage`)))
  (if _success
    (set `self.IsReturning` true)
    (elif (== OtherActor (`self.GetInstigator`))
      (`self.K2_DestroyActor`))))

(fn `UserConstructionScript`
  (`parent.UserConstructionScript`))