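; BP_BlackHole is a black hole attack projectile that pulls nearby actors toward its center.
; Its MagnetArea sphere, sized by MagnetRadius in the construction script, tracks overlapping actors other than the instigator.
; Each tick, VInterpTo moves tracked actors toward the black hole without sweeping, using an interp speed inversely proportional to distance and clamped between minimum and maximum values.
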(event `self.ReceiveTick`
  (params (DeltaSeconds :type "Float (single-precision)"))
  (`parent.ReceiveTick` DeltaSeconds)
  (for _array_element (`self.EnemiesInMagnetRange`)
    (bind _returnvalue (- (`self.K2_GetActorLocation`) (`self.K2_GetActorLocation` _array_element)))
    (set `self.EnemyDistanceWithBlackHole` (`KismetMathLibrary.VSize` _returnvalue))
    (set `self.EnemyDirection` (`KismetMathLibrary.Normal` _returnvalue))
    (bind _output_get (set `self.EnemyMagnettingSpeed` (`KismetMathLibrary.FClamp` (/ (/ (`self.MagnetRadius`) 2.0) (`self.EnemyDistanceWithBlackHole`)) (`self.MinEnemySpeed`) (`self.MaxEnemySpeed`))))
    (`self.K2_SetActorLocation` _array_element (`KismetMathLibrary.VInterpTo` (`self.K2_GetActorLocation` _array_element) (`self.K2_GetActorLocation`) DeltaSeconds _output_get) false false)))

(event `self.MagnetArea.OnComponentBeginOverlap`
  (params (OverlappedComponent :type "PrimitiveComponent Object Reference") (OtherActor :type "Actor Object Reference") (OtherComp :type "PrimitiveComponent Object Reference") (OtherBodyIndex :type Integer) (bFromSweep :type Boolean) (SweepResult :type "HitResult Structure (by ref)"))
  (if (!= OtherActor (`self.GetInstigator`))
    (`KismetArrayLibrary.Array_AddUnique` (`self.EnemiesInMagnetRange`) OtherActor)))

(event `self.MagnetArea.OnComponentEndOverlap`
  (params (OverlappedComponent :type "PrimitiveComponent Object Reference") (OtherActor :type "Actor Object Reference") (OtherComp :type "PrimitiveComponent Object Reference") (OtherBodyIndex :type Integer))
  (if (!= OtherActor (`self.GetInstigator`))
    (`KismetArrayLibrary.Array_RemoveItem` (`self.EnemiesInMagnetRange`) OtherActor)))

(fn `UserConstructionScript`
  (`parent.UserConstructionScript`)
  (`SphereComponent.SetSphereRadius` (`self.MagnetArea`) (`self.MagnetRadius`) true))