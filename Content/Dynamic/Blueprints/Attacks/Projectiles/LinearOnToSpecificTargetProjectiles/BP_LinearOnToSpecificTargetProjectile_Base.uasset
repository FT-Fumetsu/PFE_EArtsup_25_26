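; Base Blueprint for attack projectiles that fly in a straight line toward a specific target.
; On BeginPlay, after the parent logic, a valid Target triggers RotateToTarget, which sets the ProjectileMovement velocity along the direction to that target, scaled by Speed.
; The aim is taken once from the target's position at that moment, with no per-frame homing in this graph.
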(event `self.ReceiveBeginPlay`
  (`parent.ReceiveBeginPlay`)
  (`self.Target`
    (:`then`
      (`self.RotateToTarget`))
    (:`else`)))

(event `RotateToTarget`
  (set `MovementComponent.Velocity` (* (`KismetMathLibrary.GetDirectionUnitVector` (`self.K2_GetActorLocation`) (`self.K2_GetActorLocation` (`self.Target`))) (`self.Speed`)) (`self.ProjectileMovement`)))

(fn `UserConstructionScript`
  (`parent.UserConstructionScript`))