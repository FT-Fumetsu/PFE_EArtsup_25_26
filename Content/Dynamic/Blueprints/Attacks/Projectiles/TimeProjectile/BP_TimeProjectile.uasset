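; Time projectile attack that damages the enemy it overlaps, destroys itself and slows its target.
; On destruction, if the instigator has the active Singularity tag, it spawns a time dilatation area at the enemy's location.
; Event Horizon stacks widen that area, and Singularity stacks scale its slow magnitude.
; Otherwise, it applies a slow debuff to the hit enemy through set-by-caller magnitude and duration.
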(event `self.ReceiveBeginPlay`
  (`parent.ReceiveBeginPlay`))

(event `self.SphereCollider.OnComponentBeginOverlap`
  (params (OverlappedComponent :type "PrimitiveComponent Object Reference") (OtherActor :type "Actor Object Reference") (OtherComp :type "PrimitiveComponent Object Reference") (OtherBodyIndex :type Integer) (bFromSweep :type Boolean) (SweepResult :type "HitResult Structure (by ref)"))
  (set `self.EnemyLocation` (`self.K2_GetActorLocation` OtherActor))
  (bind _success (`self.CheckOverlappedActorIsEnemy` OtherActor (`self.Damage`)))
  (if _success
    (`self.K2_DestroyActor`)))

(event `self.ReceiveDestroyed`
  (bind _overlappedactorasc (`self.OverlappedActorASC`))
  (bind _returnvalue (`AbilitySystemBlueprintLibrary.GetAbilitySystemComponent` (`self.GetInstigator`)))
  (if (`GameplayTagAssetInterface.HasMatchingGameplayTag` _returnvalue (struct :`TagName` "Upgrade.Singularity.Active"))
    (set `self.Area Radius` (+ (* (`self.BonusAreaSizePerStack`) (`AbilitySystemComponent.GetGameplayEffectCount` _returnvalue "/Game/Dynamic/Blueprints/Powerups/TimeControlUpgrade/EventHorizon/GE_EventHorizon.GE_EventHorizon_C" null true)) (`self.BaseAreaRadius`)))
    (`self.SpawnSlowArea`)
    (else
      (`/Engine/EditorBlueprintResources/StandardMacros.IsValid` _overlappedactorasc
        (:`Is Valid`
          (bind _returnvalue_2 (`AbilitySystemBlueprintLibrary.AssignTagSetByCallerMagnitude` (`AbilitySystemComponent.MakeOutgoingSpec` :`self` _overlappedactorasc :`GameplayEffectClass` "/Game/Dynamic/Blueprints/Attacks/Projectiles/TimeProjectile/GE_TimeProjectileDebuff.GE_TimeProjectileDebuff_C") (struct :`TagName` "Debuff.Speed.Value") (`self.SlowDebuffMultiplier`)))
          (bind _returnvalue_3 (`AbilitySystemBlueprintLibrary.AssignTagSetByCallerMagnitude` _returnvalue_2 (struct :`TagName` "Debuff.Speed.Duration") (`self.SlowStunDuration`)))
          (`AbilitySystemComponent.BP_ApplyGameplayEffectSpecToSelf` _overlappedactorasc _returnvalue_3)))))
  (`parent.ReceiveDestroyed`))

(event `SpawnSlowArea`
  (bind (_enemylocation_x _enemylocation_y) (`KismetMathLibrary.BreakVector` (`self.EnemyLocation`)))
  (`|SpawnActorFromClass` "/Game/Dynamic/Blueprints/Powerups/TimeControlUpgrade/TimeDilatation/BP_TimeDilatationArea.BP_TimeDilatationArea_C" (`KismetMathLibrary.MakeTransform` (`KismetMathLibrary.MakeVector` _enemylocation_x _enemylocation_y)) "Undefined" "MultiplyWithRoot" null (`self.Area Radius`) "/Game/Dynamic/Blueprints/Powerups/TimeControlUpgrade/TimeDilatation/GE_TimeDilatationEnemyDebuff.GE_TimeDilatationEnemyDebuff_C" (struct :`TagName` "Data.Slow") (+ (* (- (`AbilitySystemComponent.GetGameplayEffectCount` (`AbilitySystemBlueprintLibrary.GetAbilitySystemComponent` (`self.GetInstigator`)) "/Game/Dynamic/Blueprints/Powerups/TimeControlUpgrade/Singularity/GE_SingularityGrantTag.GE_SingularityGrantTag_C" null true) 1) (`self.SlowAreaUpgradeMagnitude`)) (`self.SlowAreaMagnitude`)) (`self.AreaLifeTime`) (`GameplayStatics.GetPlayerCharacter` 0)))

(fn `UserConstructionScript`
  (`parent.UserConstructionScript`))