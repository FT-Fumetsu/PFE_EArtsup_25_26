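; Ice projectile attack Blueprint with a main sphere collider and two smaller ones that each hit independently.
; Each overlap calls OnProjectileOverlap, then passes damage to CheckOverlappedActorIsEnemy: full for the main sphere, half for the small ones.
; On an enemy hit, only that collider and its child components are destroyed, not the whole actor.
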(event `self.ReceiveTick`
  (params (DeltaSeconds :type "Float (single-precision)"))
  (`parent.ReceiveTick` DeltaSeconds))

(event `OverlapComponent`
  (params (OtherActor :type "Actor Object Reference") (DamageMagnitude :type "Float (double-precision)") (Component :type "SceneComponent Object Reference"))
  (bind _success (`self.CheckOverlappedActorIsEnemy` OtherActor DamageMagnitude))
  (if _success
    (`self.LoopDestoryComponents` Component)))

(event `self.SphereCollider.OnComponentBeginOverlap`
  (params (OverlappedComponent :type "PrimitiveComponent Object Reference") (OtherActor :type "Actor Object Reference") (OtherComp :type "PrimitiveComponent Object Reference") (OtherBodyIndex :type Integer) (bFromSweep :type Boolean) (SweepResult :type "HitResult Structure (by ref)"))
  (`self.OnProjectileOverlap` OverlappedComponent OtherComp)
  (`self.OverlapComponent` OtherActor (`self.Damage`) (`self.SphereCollider`)))

(event `self.SmallSphereCollider1.OnComponentBeginOverlap`
  (params (OverlappedComponent :type "PrimitiveComponent Object Reference") (OtherActor :type "Actor Object Reference") (OtherComp :type "PrimitiveComponent Object Reference") (OtherBodyIndex :type Integer) (bFromSweep :type Boolean) (SweepResult :type "HitResult Structure (by ref)"))
  (`self.OnProjectileOverlap` OverlappedComponent OtherComp)
  (`self.OverlapComponent` OtherActor (/ (`self.Damage`) 2.0) (`self.SmallSphereCollider1`)))

(event `self.SmallSphereCollider2.OnComponentBeginOverlap`
  (params (OverlappedComponent :type "PrimitiveComponent Object Reference") (OtherActor :type "Actor Object Reference") (OtherComp :type "PrimitiveComponent Object Reference") (OtherBodyIndex :type Integer) (bFromSweep :type Boolean) (SweepResult :type "HitResult Structure (by ref)"))
  (`self.OnProjectileOverlap` OverlappedComponent OtherComp)
  (`self.OverlapComponent` OtherActor (/ (`self.Damage`) 2.0) (`self.SmallSphereCollider2`)))

(event `LoopDestoryComponents`
  (params (Component :type "SceneComponent Object Reference"))
  (bind _output_get (set `self.TemporaryComponentArray_0` (`SceneComponent.GetChildrenComponents` Component true)))
  (for _array_element _output_get
    (`ActorComponent.K2_DestroyComponent` _array_element))
  (`ActorComponent.K2_DestroyComponent` Component))

(fn `UserConstructionScript`
  (`parent.UserConstructionScript`))