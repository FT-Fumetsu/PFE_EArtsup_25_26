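; Projectile Blueprint that homes in on a Target actor and damages what it hits.
; On BeginPlay it turns on ProjectileMovement homing toward the Target's root component, or prints a red error if the Target is invalid.
; Sphere collider overlaps pass the other actor and Damage to CheckOverlappedActor, and the projectile destroys itself when that check returns true.
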(event `self.ReceiveBeginPlay`
  (bind _projectilemovement (`self.ProjectileMovement`))
  (`parent.ReceiveBeginPlay`)
  (bind _target (`self.Target`)
    (:`then`
      (set `ProjectileMovementComponent.bIsHomingProjectile` true _projectilemovement)
      (set `ProjectileMovementComponent.HomingTargetComponent` (`Actor.RootComponent` _target) _projectilemovement))
    (:`else`
      (`KismetSystemLibrary.PrintString` "Homing Target is not valid !!" true true (struct :`R` 1.0 :`A` 1.0)))))

(event `self.SphereCollider.OnComponentBeginOverlap`
  (params (OverlappedComponent :type "PrimitiveComponent Object Reference") (OtherActor :type "Actor Object Reference") (OtherComp :type "PrimitiveComponent Object Reference") (OtherBodyIndex :type Integer) (bFromSweep :type Boolean) (SweepResult :type "HitResult Structure (by ref)"))
  (bind _hasasc (`self.CheckOverlappedActor` OtherActor (`self.Damage`)))
  (if _hasasc
    (`self.K2_DestroyActor`)))

(fn `UserConstructionScript`
  (`parent.UserConstructionScript`))