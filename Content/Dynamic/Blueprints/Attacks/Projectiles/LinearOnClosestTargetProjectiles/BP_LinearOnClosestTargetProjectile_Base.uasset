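; Base projectile that flies in a straight line toward the closest target found when it spawns.
; The construction script scans all BPI_Target actors except its owner and keeps the nearest within MaxSearchingRadius.
; On BeginPlay, if a target exists, RotateToTarget sets the ProjectileMovement velocity toward that target's location at Speed.
; Aim is set only once, with no homing, and RotateToTarget changes velocity rather than actor rotation.
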(event `self.ReceiveBeginPlay`
  (`parent.ReceiveBeginPlay`)
  (`self.Target`
    (:`then`
      (`self.RotateToTarget`))
    (:`else`)))

(event `RotateToTarget`
  (set `MovementComponent.Velocity` (* (`KismetMathLibrary.GetDirectionUnitVector` (`self.K2_GetActorLocation`) (`self.K2_GetActorLocation` (`self.Target`))) (`self.Speed`)) (`self.ProjectileMovement`)))

(fn `FindClosestTarget`
  (locals (ClosestDistance :type "Float (double-precision)"))
  (bind _returnvalue (`KismetMathLibrary.VSize` (- (`self.K2_GetActorLocation`) (`self.K2_GetActorLocation`))))
  (set `local.ClosestDistance` (`self.MaxSearchingRadius`))
  (bind _outactors (`GameplayStatics.GetAllActorsWithInterface` "/Game/Dynamic/Blueprints/Attacks/Projectiles/Interfaces/BPI_Target.BPI_Target_C"))
  (for _array_element _outactors
    (if (and (not (== _array_element (`self.GetOwner`))) (< _returnvalue (`local.ClosestDistance`)))
      (set `local.ClosestDistance` _returnvalue)
      (set `self.Target` _array_element))))

(fn `UserConstructionScript`
  (`parent.UserConstructionScript`)
  (set `self.Target` null)
  (`self.FindClosestTarget`))