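; BP_Landscape is a procedural landscape actor that builds a noise-driven terrain chunk and scatters foliage over it at BeginPlay.
; It spawns a single BP_Chunk, copies its size, scale, material and fractal and cellular noise settings onto it, then calls Generate.
; It then spawns BP_MeshesGenerator and passes the chunk's XY bounds and center Z to GenerateFolliage.
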(event `self.ReceiveBeginPlay`
  (bind (_origin _boxextent) (`self.GetActorBounds` (`self.Chunk`) false false))
  (bind _x (.x _boxextent))
  (bind _y (.y _boxextent))
  (bind _x_2 (.x _origin))
  (bind _y_2 (.y _origin))
  (bind _returnvalue (`|SpawnActorFromClass` "/Game/Dynamic/Blueprints/ProceduralGenerationActors/BP_Chunk.BP_Chunk_C" (`KismetMathLibrary.MakeTransform` (0.0 0.0 0.0)) "Undefined" "MultiplyWithRoot" null null))
  (bind _output_get (set `self.Chunk` _returnvalue))
  (`self.SetChunkParameters` _output_get)
  (`/Game/Dynamic/Blueprints/ProceduralGenerationActors/BP_Chunk.Generate` (`self.Chunk`))
  (bind _returnvalue_2 (`|SpawnActorFromClass` "/Game/Dynamic/Blueprints/ProceduralGenerationActors/BP_MeshesGenerator.BP_MeshesGenerator_C" (`KismetMathLibrary.MakeTransform` (0.0 0.0 0.0)) "Undefined" "MultiplyWithRoot" null null))
  (bind _output_get_2 (set `self.MeshesGenreator` _returnvalue_2))
  (`/Game/Dynamic/Blueprints/ProceduralGenerationActors/BP_MeshesGenerator.GenerateFolliage` _output_get_2 (- _x_2 _x) (+ _x_2 _x) (- _y_2 _y) (+ _y_2 _y) (.z _origin)))

(fn `SetChunkParameters`
  (params (Chunk :type "/Game/Dynamic/Blueprints/ProceduralGenerationActors/BP_Chunk Object Reference"))
  (set `/Game/Dynamic/Blueprints/ProceduralGenerationActors/BP_Chunk.Size` (`self.Size`) (`local.Chunk`))
  (set `/Game/Dynamic/Blueprints/ProceduralGenerationActors/BP_Chunk.Scale` (`self.Scale`) (`local.Chunk`))
  (set `/Game/Dynamic/Blueprints/ProceduralGenerationActors/BP_Chunk.UVScale` (`self.UVScale`) (`local.Chunk`))
  (set `/Game/Dynamic/Blueprints/ProceduralGenerationActors/BP_Chunk.ZMultiplier` (`self.ZMultiplier`) (`local.Chunk`))
  (set `/Game/Dynamic/Blueprints/ProceduralGenerationActors/BP_Chunk.Material` (`self.Material`) (`local.Chunk`))
  (set `/Game/Dynamic/Blueprints/ProceduralGenerationActors/BP_Chunk.Gain` (`self.Gain`) (`local.Chunk`))
  (set `/Game/Dynamic/Blueprints/ProceduralGenerationActors/BP_Chunk.Lacunarity` (`self.Lacunarity`) (`local.Chunk`))
  (set `/Game/Dynamic/Blueprints/ProceduralGenerationActors/BP_Chunk.Octaves` (`self.Octaves`) (`local.Chunk`))
  (set `/Game/Dynamic/Blueprints/ProceduralGenerationActors/BP_Chunk.Fractaltype` (`self.Fractaltype`) (`local.Chunk`))
  (set `/Game/Dynamic/Blueprints/ProceduralGenerationActors/BP_Chunk.Interp` (`self.Interp`) (`local.Chunk`))
  (set `/Game/Dynamic/Blueprints/ProceduralGenerationActors/BP_Chunk.Frequency` (`self.Frequency`) (`local.Chunk`))
  (set `/Game/Dynamic/Blueprints/ProceduralGenerationActors/BP_Chunk.Seed` (`self.Seed`) (`local.Chunk`))
  (set `/Game/Dynamic/Blueprints/ProceduralGenerationActors/BP_Chunk.Noise Type` (`self.Type`) (`local.Chunk`))
  (set `/Game/Dynamic/Blueprints/ProceduralGenerationActors/BP_Chunk.Cellular Return Type` (`self.ReturnType`) (`local.Chunk`))
  (set `/Game/Dynamic/Blueprints/ProceduralGenerationActors/BP_Chunk.Cellular Distance Function` (`self.DistanceFunction`) (`local.Chunk`))
  (set `/Game/Dynamic/Blueprints/ProceduralGenerationActors/BP_Chunk.Cellular Jitter` (`self.Jitter`) (`local.Chunk`)))

(fn `UserConstructionScript`)