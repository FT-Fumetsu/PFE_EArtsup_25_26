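; BP_Generator is a procedural generation actor that spawns a flat grid of BP_Cell actors on BeginPlay.
; GeneratePattern first fills a list of unique positions from Size and CellSize, starting at world origin rather than the actor's location.
; GenerateGrid spawns cells from that list while removing each used position mid-loop, and records the cells in AllCells.
; DestroyAllCells destroys and clears the recorded cells, but nothing here calls it.
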(event `DestroyAllCells`
  (bind _allcells (`self.AllCells`))
  (for _array_element _allcells
    (`self.K2_DestroyActor` _array_element))
  (`KismetArrayLibrary.Array_Clear` _allcells))

(event `self.ReceiveBeginPlay`
  (`self.GeneratePattern`))

(event `InitAvailablePositions`
  (bind (_x _y) (`KismetMathLibrary.BreakVector2D` (`self.Size`)))
  (`KismetArrayLibrary.Array_Clear` (`self.AvailaibleCells`))
  (for _index (range (`KismetMathLibrary.FTrunc` _x))
    (for _index_2 (range (`KismetMathLibrary.FTrunc` _y))
      (`KismetArrayLibrary.Array_AddUnique` (`self.AvailaibleCells`) (`KismetMathLibrary.MakeVector` (* _index (`self.CellSize`)) (* _index_2 (`self.CellSize`)))))))

(event `GenerateGrid`
  (for _array_element (`self.AvailaibleCells`)
    (bind _returnvalue (`|SpawnActorFromClass` "/Game/Dynamic/Blueprints/ProceduralGenerationActors/BP_Cell.BP_Cell_C" (`KismetMathLibrary.MakeTransform` _array_element) "AlwaysSpawn" "MultiplyWithRoot" null null))
    (`KismetArrayLibrary.Array_AddUnique` (`self.AllCells`) _returnvalue)
    (`KismetArrayLibrary.Array_RemoveItem` (`self.AvailaibleCells`) (`self.K2_GetActorLocation` _returnvalue))))

(event `GeneratePattern`
  (`self.InitAvailablePositions`)
  (`self.GenerateGrid`))

(fn `UserConstructionScript`)