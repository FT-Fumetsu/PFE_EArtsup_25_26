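; BP_MeshesGenerator scatters foliage actors over procedurally generated meshes within given XY bounds.
; GenerateFolliage picks about 500 random points and sphere-traces vertically upward through the given height against WorldStatic objects.
; Where the hit actor carries the ProceduralMesh tag, it spawns BP_TestFolliage raised above the hit location with random yaw, ignoring collisions.
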(fn `GenerateFolliage`
  (params (XMin :type "Float (double-precision)") (XMax :type "Float (double-precision)") (YMin :type "Float (double-precision)") (YMax :type "Float (double-precision)") (Z :type "Float (double-precision)"))
  (bind _positionx (`self.PositionX`))
  (bind _positiony (`self.PositionY`))
  (bind _positionz (`self.PositionZ`))
  (for _ (range 501)
    (set `self.PositionX` (`KismetMathLibrary.RandomFloatInRange` (`local.XMin`) (`local.XMax`)))
    (set `self.PositionY` (`KismetMathLibrary.RandomFloatInRange` (`local.YMin`) (`local.YMax`)))
    (set `self.PositionZ` (`local.Z`))
    (bind _outhit (`KismetSystemLibrary.SphereTraceSingleForObjects` :`Start` (`KismetMathLibrary.MakeVector` _positionx _positiony (- _positionz 2000.0)) :`End` (`KismetMathLibrary.MakeVector` _positionx _positiony (+ _positionz 2000.0)) :`Radius` 100.0 :`ObjectTypes` (`|MakeArray` "ObjectTypeQuery1" :!type "EObjectTypeQuery Enum") :`DrawTime` 2.0))
    (bind (_bblockinghit _binitialoverlap _time _distance _location _impactpoint _normal _impactnormal _physmat _hitactor) (`GameplayStatics.BreakHitResult` _outhit))
    (if (`self.ActorHasTag` _hitactor "ProceduralMesh")
      (`|SpawnActorFromClass` "/Game/Dynamic/Blueprints/ProceduralGenerationActors/BP_TestFolliage.BP_TestFolliage_C" (`KismetMathLibrary.MakeTransform` (+ _location (0.0 0.0 200.0)) (`KismetMathLibrary.MakeRotator` 0.0 0.0 (`KismetMathLibrary.RandomFloatInRange` 0.0 360.0))) "AlwaysSpawn" "MultiplyWithRoot" null null))))

(fn `UserConstructionScript`)