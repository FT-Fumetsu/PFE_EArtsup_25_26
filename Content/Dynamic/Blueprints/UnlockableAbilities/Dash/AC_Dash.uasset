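; AC_Dash is a dash component for an unlockable ability that shifts its owning actor forward.
; DashBegin plays the dash montage and immediately passes a point DashDistance ahead to MoveOverTime.
; MoveOverTime faces the owner toward that point and teleports it, without sweeping, to a lerp between start and target.
; Despite the name, the move is a single step: nothing here animates LocationAlpha.
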(event `DashBegin`
  (bind _returnvalue (`self.GetOwner`))
  (`|PlayMontage` (`self.Mesh`) (`self.DashMontage`)
    (:`then`
      (`self.MoveOverTime` (+ (`Actor.K2_GetActorLocation` _returnvalue) (* (`Actor.GetActorForwardVector` _returnvalue) (`self.DashDistance`)))))))

(event `MoveOverTime`
  (params (Location :type "Vector Structure"))
  (bind _returnvalue (`self.GetOwner`))
  (bind _output_get (set `self.DashStartLocation` (`Actor.K2_GetActorLocation` _returnvalue)))
  (`Actor.K2_SetActorRotation` _returnvalue (`KismetMathLibrary.FindLookAtRotation` _output_get Location) false)
  (`Actor.K2_SetActorLocation` (`self.GetOwner`) (`KismetMathLibrary.VLerp` (`self.DashStartLocation`) Location (`self.LocationAlpha`)) false true))