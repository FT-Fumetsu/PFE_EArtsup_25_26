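; Dash damage powerup upgrade, named as a base class, that supplies the effect magnitude to inherited upgrade logic.
; On BeginPlay it runs the parent setup, sets a fixed EffectMagnitudeValue, then immediately calls ApplyUpgrade.
; Its ApplyUpgrade only forwards to the parent, so this Blueprint does not define how the magnitude affects dash damage.
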(event `self.ReceiveBeginPlay`
  (`parent.ReceiveBeginPlay`)
  (set `self.EffectMagnitudeValue` 50.0)
  (`self.ApplyUpgrade`))

(event `self.ApplyUpgrade`
  (`parent.ApplyUpgrade`))

(fn `UserConstructionScript`
  (`parent.UserConstructionScript`))