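; Base speed upgrade powerup that applies a Gameplay Ability System effect to the player as soon as it spawns.
; BeginPlay copies the speed upgrade value into the inherited effect magnitude, then calls ApplyUpgrade.
; ApplyUpgrade runs the parent logic, then applies the effect class to player 0 with that magnitude set by caller tag.
; A debug print then shows MaxHealth rather than a speed attribute.
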(event `self.ReceiveBeginPlay`
  (`parent.ReceiveBeginPlay`)
  (set `self.EffectMagnitudeValue` (`self.SpeedUpgradeValue`))
  (`self.ApplyUpgrade`))

(event `self.ApplyUpgrade`
  (bind _returnvalue (`GameplayStatics.GetPlayerCharacter` 0))
  (bind _returnvalue_2 (`AbilitySystemBlueprintLibrary.GetAbilitySystemComponent` _returnvalue))
  (bind (_maxhealth_basevalue _maxhealth_currentvalue) (break `GameplayAttributeData` (`BasicAttributeSet.MaxHealth` (`GASCharacterBase.BasicAttributeSet` (cast `/Game/Dynamic/Blueprints/Controllers/Player/BP_Player` _returnvalue :!pure true)))))
  (`parent.ApplyUpgrade`)
  (`/Engine/EditorBlueprintResources/StandardMacros.IsValid` _returnvalue_2
    (:`Is Valid`
      (bind _returnvalue_3 (`AbilitySystemBlueprintLibrary.MakeSpecHandleByClass` (`self.EffectClass`) null self))
      (bind _returnvalue_4 (`AbilitySystemBlueprintLibrary.AssignTagSetByCallerMagnitude` _returnvalue_3 (`self.EffectMagnitudeDataType`) (`self.EffectMagnitudeValue`)))
      (`AbilitySystemComponent.BP_ApplyGameplayEffectSpecToSelf` _returnvalue_2 _returnvalue_4)
      (`KismetSystemLibrary.PrintString` (`KismetStringLibrary.Concat_StrStr` "MaxHealth = " (`KismetStringLibrary.Conv_DoubleToString` _maxhealth_currentvalue))))))

(fn `UserConstructionScript`
  (`parent.UserConstructionScript`))