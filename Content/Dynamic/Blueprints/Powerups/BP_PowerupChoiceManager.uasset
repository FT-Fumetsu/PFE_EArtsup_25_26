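; Manager that offers the player a weighted random choice of powerups in a chest widget.
; ChooseUpgrades filters candidates by prerequisite upgrade, GAS attribute limits and stack count, then draws unique picks using cumulative rarity weights.
; It opens WBP_Chest with the picks, pauses the game and binds the widget's click event.
; ApplyUpgrade applies a powerup by spawning its class as an actor.
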(event `self.ReceiveBeginPlay`
  (set `self.PlayerRef` (`GameplayStatics.GetPlayerCharacter` 0)))

(event `ChooseUpgrades`
  (params (UpgradeArray :type "Array of /Game/Dynamic/Blueprints/Powerups/BP_BaseUpgrade Class Reference") (ChoiceCount :type Integer))
  (bind _availableupgradearray (`self.AvailableUpgradeArray`))
  (bind _output_get (set `self.AvailableUpgradeArray` UpgradeArray))
  (`KismetArrayLibrary.Array_Clear` (`self.SelectedUpgrades`))
  (for _array_element _output_get
    (bind _canbepicked (`self.UpgradeCanBePicked` _array_element))
    (if (not _canbepicked)
      (`KismetArrayLibrary.Array_RemoveItem` _availableupgradearray _array_element)))
  (while (and (< (`KismetArrayLibrary.Array_Length` (`self.SelectedUpgrades`)) ChoiceCount) (`KismetArrayLibrary.Array_IsNotEmpty` (`self.AvailableUpgradeArray`)))
    (`self.ChoosePowerup` _availableupgradearray))
  (`self.OpenWidget`))

(event `ApplyUpgrade`
  (params (RowPowerUp :type "/Game/Dynamic/Blueprints/Powerups/BP_BaseUpgrade Class Reference"))
  (`|SpawnActorFromClass` RowPowerUp (`KismetMathLibrary.MakeTransform` (0.0 0.0 0.0)) "AlwaysSpawn" "MultiplyWithRoot" null null))

(fn `ChoosePowerup`
  (params (AvailableUpgrades :type "Array of /Game/Dynamic/Blueprints/Powerups/BP_BaseUpgrade Class Reference"))
  (set `self.TotalWeight` 0)
  (for _array_element AvailableUpgrades
    (set `self.TotalWeight` (+ (`self.TotalWeight`) (`self.GetRarityWeight` (`.Rarity_20_C33BCB9F400591889A4ECCB9557C33BB` (break `/Game/Dynamic/Blueprints/Structures/PowerUps/Str_PowerUps` (defaults `Object` _array_element)))))))
  (`self.CumulativeCalculation` AvailableUpgrades))

(fn `CumulativeCalculation`
  (params (AvailableUpgrades :type "Array of /Game/Dynamic/Blueprints/Powerups/BP_BaseUpgrade Class Reference"))
  (bind _output_get (set `self.RandomWeight` (`KismetMathLibrary.RandomIntegerInRange` 0 (`self.TotalWeight`))))
  (for _array_element AvailableUpgrades
    (bind _output_get_2 (set `self.CumulativeWeight` (+ (`self.CumulativeWeight`) (`self.GetRarityWeight` (`.Rarity_20_C33BCB9F400591889A4ECCB9557C33BB` (break `/Game/Dynamic/Blueprints/Structures/PowerUps/Str_PowerUps` (defaults `Object` _array_element)))))))
    (if (>= _output_get_2 (`self.RandomWeight`))
      (`KismetArrayLibrary.Array_AddUnique` (`self.SelectedUpgrades`) _array_element)
      (`KismetArrayLibrary.Array_RemoveItem` (`self.AvailableUpgradeArray`) _array_element)
      (set `self.CumulativeWeight` 0)
      (break))))

(fn `GetRarityWeight`
  (params (Rarity :type "/Game/Dynamic/Blueprints/Enums/PowerUps/E_PowerUpsRarity Enum" :default "NewEnumerator0"))
  (returns (Weight :type Integer))
  (switch `/Game/Dynamic/Blueprints/Enums/PowerUps/E_PowerUpsRarity` Rarity
    (:`NewEnumerator0`
      (return 30))
    (:`NewEnumerator1`
      (return 15))
    (:`NewEnumerator2`
      (return 10))
    (:`NewEnumerator3`
      (return 6))
    (:`NewEnumerator4`
      (return 3))
    (:`NewEnumerator5`
      (return 1))))

(fn `IsPlayerHasAllUpgraadeCount`
  (params (Powerup :type "/Game/Dynamic/Blueprints/Powerups/BP_BaseUpgrade Class Reference"))
  (returns (CanBePick :type Boolean))
  (locals (NumberOfThisUpgradeInPlayer :type Integer))
  (for _array_element (`/Game/Dynamic/Blueprints/Controllers/Player/BP_Player.AllObtainedUpgrades` (cast `/Game/Dynamic/Blueprints/Controllers/Player/BP_Player` (`GameplayStatics.GetPlayerCharacter` 0) :!pure true))
    (if (== _array_element Powerup)
      (set `local.NumberOfThisUpgradeInPlayer` (+ (`local.NumberOfThisUpgradeInPlayer`) 1))))
  (return (<= (`local.NumberOfThisUpgradeInPlayer`) (`.MaxStack_25_D53BB2B748726CA5081F379A725EB6BD` (break `/Game/Dynamic/Blueprints/Structures/PowerUps/Str_PowerUps` (defaults `Object` Powerup))))))

(fn `IsPlayerHasDependentUpgrade`
  (params (PowerupData :type "/Game/Dynamic/Blueprints/Structures/PowerUps/Str_PowerUps Structure"))
  (returns (CanBePicked :type Boolean))
  (bind ((`IsUpgrade?_11_4C7A76A444154D8209EAA685AF69CB9F` _isupgrade_) (`UpgradeTarget_49_8CB1110440DBD9F2DA118898BA61B50D` _upgradetarget)) (break `/Game/Dynamic/Blueprints/Structures/PowerUps/Str_PowerUps` PowerupData))
  (if _isupgrade_
    (return (`KismetArrayLibrary.Array_Contains` (`/Game/Dynamic/Blueprints/Controllers/Player/BP_Player.AllObtainedUpgrades` (cast `/Game/Dynamic/Blueprints/Controllers/Player/BP_Player` (`GameplayStatics.GetPlayerCharacter` 0) :!pure true)) _upgradetarget))
    (else
      (return true))))

(fn `OpenWidget`
  (bind _returnvalue (`GameplayStatics.GetPlayerController` 0))
  (bind _returnvalue_2 (`|CreateWidget` "/Game/Dynamic/Blueprints/WidgetBlueprint(WBP)/Chests/WBP_Chest.WBP_Chest_C"))
  (`UserWidget.AddToViewport` _returnvalue_2 0)
  (set `PlayerController.bShowMouseCursor` true _returnvalue)
  (`WidgetBlueprintLibrary.SetInputMode_UIOnlyEx` _returnvalue null)
  (`MovementComponent.StopMovementImmediately` (`Character.CharacterMovement` (cast `/Game/Dynamic/Blueprints/Controllers/Player/BP_Player` (`self.PlayerRef`) :!pure true)))
  (`GameplayStatics.SetGamePaused` true)
  (`/Game/Dynamic/Blueprints/WidgetBlueprint(WBP)/Chests/WBP_Chest.InitializeCoices` _returnvalue_2 (`self.SelectedUpgrades`))
  (add `/Game/Dynamic/Blueprints/WidgetBlueprint(WBP)/Chests/WBP_Chest.OnChoiceClicked` _returnvalue_2 (`|CreateDelegate` :!event `ApplyUpgrade`)))

(fn `StatCanBeUpgrade`
  (params (PowerupData :type "/Game/Dynamic/Blueprints/Structures/PowerUps/Str_PowerUps Structure"))
  (returns (CanBeUpgrade :type Boolean))
  (bind ((`UpgradeValue_48_3119941241861E6C07779589B2946D26` _upgradevalue) (`IsDependantOnStat_34_26DB8FD24EC781D56B9EA08E6D44C98E` _isdependantonstat) (`StatDependency_43_36E4D15A4C5DB0B9399457AA0E8BA74B` _statdependency) (`MaxStatDependency_44_56A63275434ABC9F353E888BB9C6F32A` _maxstatdependency) (`MinStatDependency_45_8FCC6F99410B56511C2E658D2220FA30` _minstatdependency)) (break `/Game/Dynamic/Blueprints/Structures/PowerUps/Str_PowerUps` PowerupData))
  (bind _returnvalue (`AbilitySystemBlueprintLibrary.GetAbilitySystemComponent` (`GameplayStatics.GetPlayerCharacter` 0)))
  (bind (_bsuccessfullyfoundattribute _returnvalue_2) (`AbilitySystemBlueprintLibrary.GetFloatAttributeFromAbilitySystemComponent` _returnvalue _statdependency))
  (if _isdependantonstat
    (if (> _upgradevalue 0.0)
      (if (`AbilitySystemBlueprintLibrary.IsValid` _maxstatdependency)
        (if (< _returnvalue_2 (`.ReturnValue` (`AbilitySystemBlueprintLibrary.GetFloatAttributeFromAbilitySystemComponent` _returnvalue _maxstatdependency)))
          _
          (else
            (return false))))
      (elif (> _returnvalue_2 (`.ReturnValue` (`AbilitySystemBlueprintLibrary.GetFloatAttributeFromAbilitySystemComponent` _returnvalue _minstatdependency)))
        _
        (else
          (return false))))
    (return true)
    (else
      (return true))))

(fn `UpgradeCanBePicked`
  (params (PowerupData :type "/Game/Dynamic/Blueprints/Powerups/BP_BaseUpgrade Class Reference"))
  (returns (CanBePicked :type Boolean))
  (bind _powerupdata (defaults `Object` PowerupData))
  (bind _canbepicked (`self.IsPlayerHasDependentUpgrade` _powerupdata))
  (if _canbepicked
    (bind _canbeupgrade (`self.StatCanBeUpgrade` _powerupdata))
    (if _canbeupgrade
      (bind _canbepick (`self.IsPlayerHasAllUpgraadeCount` PowerupData))
      (if _canbepick
        (return true)
        (else
          _))))
  (return false))

(fn `UserConstructionScript`)