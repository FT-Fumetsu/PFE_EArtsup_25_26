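; BP_TimeDilatationArea is a spherical area actor for the time dilatation part of the Time Control powerup upgrade.
; Its construction script runs the parent's, then sizes the Sphere component from AreaRadius.
; Begin and end overlap events pass to the parent class for every actor except the Instigator, which keeps the Instigator out of the inherited area logic.
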(event `self.ReceiveActorBeginOverlap`
  (params (OtherActor :type "Actor Object Reference"))
  (if (!= OtherActor (`self.GetInstigator`))
    (`parent.ReceiveActorBeginOverlap` OtherActor)))

(event `self.ReceiveActorEndOverlap`
  (params (OtherActor :type "Actor Object Reference"))
  (if (!= OtherActor (`self.GetInstigator`))
    (`parent.ReceiveActorEndOverlap` OtherActor)))

(fn `UserConstructionScript`
  (`parent.UserConstructionScript`)
  (`SphereComponent.SetSphereRadius` (`self.Sphere`) (`self.AreaRadius`) true))