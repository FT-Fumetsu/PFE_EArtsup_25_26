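; Time dilatation powerup that gives the player an area applying a slow debuff to enemies, applied on BeginPlay.
; The first application spawns BP_TimeDilatationArea attached to the player and builds a player debuff spec with SetByCaller duration and value, without applying it in this graph.
; Later applications add a radius GameplayEffect and resize the existing sphere from the effect count, using GAS to track upgrades.
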(event `self.ReceiveBeginPlay`
  (`parent.ReceiveBeginPlay`)
  (`self.ApplyUpgrade`))

(event `self.ApplyUpgrade`
  (bind _returnvalue (`GameplayStatics.GetPlayerCharacter` 0))
  (bind (_returnvalue_location _returnvalue_rotation _returnvalue_scale) (`KismetMathLibrary.BreakTransform` (`self.GetTransform` _returnvalue)))
  (bind _returnvalue_2 (`AbilitySystemBlueprintLibrary.GetAbilitySystemComponent` _returnvalue))
  (bind _timedilatationarea (`/Game/Dynamic/Blueprints/Controllers/Player/BP_Player.TimeDilatationArea` (cast `/Game/Dynamic/Blueprints/Controllers/Player/BP_Player` _returnvalue :!pure true)))
  (`/Engine/EditorBlueprintResources/StandardMacros.IsValid` _timedilatationarea
    (:`Is Valid`
      (`AbilitySystemComponent.BP_ApplyGameplayEffectToSelf` :`self` _returnvalue_2 :`GameplayEffectClass` "/Game/Dynamic/Blueprints/Powerups/TimeControlUpgrade/TimeDilatation/GE_TimeDilatationAreaRadius.GE_TimeDilatationAreaRadius_C")
      (`SphereComponent.SetSphereRadius` (`/Game/Dynamic/Blueprints/GameplayAbilitySystem/EffectActors/BP_EffectArea_Base.Sphere` _timedilatationarea) (+ (`self.Area Radius`) (* (`AbilitySystemComponent.GetGameplayEffectCount` _returnvalue_2 null null true) (`self.AreaUpgradeValue`))) true))
    (:`Is Not Valid`
      (bind _returnvalue_3 (`|SpawnActorFromClass` "/Game/Dynamic/Blueprints/Powerups/TimeControlUpgrade/TimeDilatation/BP_TimeDilatationArea.BP_TimeDilatationArea_C" (`KismetMathLibrary.MakeTransform` _returnvalue_location _returnvalue_rotation _returnvalue_scale) "Undefined" "MultiplyWithRoot" null (`self.Area Radius`) "/Game/Dynamic/Blueprints/Powerups/TimeControlUpgrade/TimeDilatation/GE_TimeDilatationEnemyDebuff.GE_TimeDilatationEnemyDebuff_C" (struct :`TagName` "Data.Slow") (`self.Effect Magnitude Value`) 0.0 _returnvalue))
      (`SceneComponent.K2_AddLocalOffset` (`/Game/Dynamic/Blueprints/Powerups/TimeControlUpgrade/TimeDilatation/BP_TimeDilatationArea.VFX_0` _returnvalue_3) (0.0 0.0 -80.0) false false)
      (`self.K2_AttachToComponent` _returnvalue_3 (`Actor.RootComponent` _returnvalue) "None" "KeepWorld" "KeepWorld" "KeepWorld" true)
      (bind _returnvalue_4 (`AbilitySystemBlueprintLibrary.AssignTagSetByCallerMagnitude` (`AbilitySystemComponent.MakeOutgoingSpec` :`self` _returnvalue_2 :`GameplayEffectClass` "/Game/Dynamic/Blueprints/Powerups/TimeControlUpgrade/TimeDilatation/GE_TimeDilatationPlayerDebuff.GE_TimeDilatationPlayerDebuff_C") (struct :`TagName` "Upgrade.TimeDilatation.Player.Duration") (`self.DebuffDuration`)))
      (`AbilitySystemBlueprintLibrary.AssignTagSetByCallerMagnitude` _returnvalue_4 (struct :`TagName` "Upgrade.TimeDilatation.Player.Value") (`self.Effect Magnitude Value`))
      (`parent.ApplyUpgrade`))))

(fn `UserConstructionScript`
  (`parent.UserConstructionScript`))