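; BP_ZaWarudo is a time-control powerup upgrade that gives the player the ZaWarudo ability.
; On BeginPlay it calls its ApplyUpgrade event, which applies the GE_Upgrade_ZaWarudo gameplay effect and grants GA_ZaWarudo through player 0's Ability System Component.
; It then calls the parent ApplyUpgrade, so any shared upgrade logic comes from the parent class.
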(event `self.ReceiveBeginPlay`
  (`parent.ReceiveBeginPlay`)
  (`self.ApplyUpgrade`))

(event `self.ApplyUpgrade`
  (bind _returnvalue (`AbilitySystemBlueprintLibrary.GetAbilitySystemComponent` (`GameplayStatics.GetPlayerCharacter` 0)))
  (`AbilitySystemComponent.BP_ApplyGameplayEffectToSelf` :`self` _returnvalue :`GameplayEffectClass` "/Game/Dynamic/Blueprints/Powerups/TimeControlUpgrade/GE_Upgrade_ZaWarudo.GE_Upgrade_ZaWarudo_C")
  (`AbilitySystemComponent.K2_GiveAbility` _returnvalue "/Game/Dynamic/Blueprints/Powerups/TimeControlUpgrade/GA_ZaWarudo.GA_ZaWarudo_C" 0 -1)
  (`parent.ApplyUpgrade`))

(fn `UserConstructionScript`
  (`parent.UserConstructionScript`))