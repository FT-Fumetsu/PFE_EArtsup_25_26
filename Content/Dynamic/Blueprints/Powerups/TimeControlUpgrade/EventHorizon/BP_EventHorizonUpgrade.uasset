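; BP_EventHorizonUpgrade is the Event Horizon powerup upgrade, filed under the time control upgrades.
; On BeginPlay it calls ApplyUpgrade, which applies the GE_EventHorizon gameplay effect to player 0's ability system component, then runs the parent's ApplyUpgrade.
; The upgrade's behavior comes from that effect and the parent class, as the overlap and tick events are disabled.
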(event `self.ReceiveBeginPlay`
  (`parent.ReceiveBeginPlay`)
  (`self.ApplyUpgrade`))

(event `self.ApplyUpgrade`
  (`AbilitySystemComponent.BP_ApplyGameplayEffectToSelf` :`self` (`AbilitySystemBlueprintLibrary.GetAbilitySystemComponent` (`GameplayStatics.GetPlayerCharacter` 0)) :`GameplayEffectClass` "/Game/Dynamic/Blueprints/Powerups/TimeControlUpgrade/EventHorizon/GE_EventHorizon.GE_EventHorizon_C")
  (`parent.ApplyUpgrade`))

(fn `UserConstructionScript`
  (`parent.UserConstructionScript`))