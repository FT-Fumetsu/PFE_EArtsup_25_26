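; Gameplay ability for the Za Warudo time-control upgrade, which heals the player and slows the world around them for a limited time.
; It applies a heal effect scaled from max health, then sets global dilation to the inverse of the player's custom dilation, keeping the player at normal speed.
; A per-tick real-time check restores both dilations and ends the ability, which removes effects granting the upgrade tag.
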(event `self.K2_ActivateAbility`
  (bind _returnvalue (`self.GetAvatarActorFromActorInfo`))
  (bind _timedilatation (`self.TimeDilatation`))
  (bind _asbp_player (cast `/Game/Dynamic/Blueprints/Controllers/Player/BP_Player` _returnvalue :!pure true))
  (bind (_maxhealth_basevalue _maxhealth_currentvalue) (break `GameplayAttributeData` (`BasicAttributeSet.MaxHealth` (`GASCharacterBase.BasicAttributeSet` _asbp_player))))
  (bind _returnvalue_2 (`AbilitySystemBlueprintLibrary.AssignTagSetByCallerMagnitude` (`self.MakeOutgoingGameplayEffectSpec` "/Game/Dynamic/Blueprints/Powerups/TimeControlUpgrade/ZaWarudo/GE_ZaWarudoHeal.GE_ZaWarudoHeal_C") (struct :`TagName` "Statistics.Add.Health") (* _maxhealth_currentvalue (`self.MultiplierHealing`))))
  (`AbilitySystemComponent.BP_ApplyGameplayEffectSpecToSelf` (`AbilitySystemBlueprintLibrary.GetAbilitySystemComponent` _returnvalue) _returnvalue_2)
  (set `self.RealTimeBeforeTimeStops` (`GameplayStatics.GetRealTimeSeconds`))
  (set `Actor.CustomTimeDilation` _timedilatation _asbp_player)
  (set `Actor.CustomTimeDilation` _timedilatation _returnvalue)
  (`GameplayStatics.SetGlobalTimeDilation` (/ 1.0 (`self.TimeDilatation`)))
  (if (>= (- (`GameplayStatics.GetRealTimeSeconds`) (`self.RealTimeBeforeTimeStops`)) (`self.TimeBeforeFreezeStops`)) :!label _label
    (set `Actor.CustomTimeDilation` 1.0 _returnvalue)
    (`GameplayStatics.SetGlobalTimeDilation` 1.0)
    (`self.K2_EndAbility`)
    (else
      (`KismetSystemLibrary.DelayUntilNextTick`)
      (goto _label))))

(event `self.K2_OnEndAbility`
  (params (bWasCancelled :type Boolean))
  (`AbilitySystemComponent.RemoveActiveEffectsWithGrantedTags` (`AbilitySystemBlueprintLibrary.GetAbilitySystemComponent` (`self.GetAvatarActorFromActorInfo`)) (struct :`GameplayTags` (struct :`(TagName` "Upgrade.ZaWarudo")))))