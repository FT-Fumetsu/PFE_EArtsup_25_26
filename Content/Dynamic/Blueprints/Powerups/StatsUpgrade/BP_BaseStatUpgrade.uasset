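; Base Blueprint for stat upgrade powerups that applies a Gameplay Effect to the player when the upgrade is applied.
; ApplyUpgrade gets the first player character's Ability System Component and, if valid, builds a spec from EffectClass with this actor as causer.
; A tag-driven SetByCaller magnitude makes the effect data-configurable, and the parent ApplyUpgrade runs only after the spec is applied.
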(event `self.ApplyUpgrade`
  (bind _returnvalue (`AbilitySystemBlueprintLibrary.GetAbilitySystemComponent` (`GameplayStatics.GetPlayerCharacter` 0)))
  (`/Engine/EditorBlueprintResources/StandardMacros.IsValid` _returnvalue
    (:`Is Valid`
      (bind _returnvalue_2 (`AbilitySystemBlueprintLibrary.MakeSpecHandleByClass` (`self.EffectClass`) null self))
      (bind _returnvalue_3 (`AbilitySystemBlueprintLibrary.AssignTagSetByCallerMagnitude` _returnvalue_2 (`self.EffectMagnitudeDataType`) (`self.EffectMagnitudeValue`)))
      (`AbilitySystemComponent.BP_ApplyGameplayEffectSpecToSelf` _returnvalue _returnvalue_3)
      (`parent.ApplyUpgrade`))))

(fn `UserConstructionScript`
  (`parent.UserConstructionScript`))