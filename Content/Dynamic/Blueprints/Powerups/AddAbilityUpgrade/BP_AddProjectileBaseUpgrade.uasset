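; Powerup upgrade Blueprint in the AddAbilityUpgrade family, named for adding a base projectile upgrade.
; On BeginPlay it casts the player character to BP_Player and stores its ProjectileColliderRange as OverlappingZone before running the parent's BeginPlay.
; ApplyUpgrade only forwards to the parent class, so the upgrade behavior itself is inherited.
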(event `self.ReceiveBeginPlay`
  (set `self.OverlappingZone` (`/Game/Dynamic/Blueprints/Controllers/Player/BP_Player.ProjectileColliderRange` (cast `/Game/Dynamic/Blueprints/Controllers/Player/BP_Player` (`GameplayStatics.GetPlayerCharacter` 0) :!pure true)))
  (`parent.ReceiveBeginPlay`))

(event `self.ApplyUpgrade`
  (`parent.ApplyUpgrade`))

(fn `UserConstructionScript`
  (`parent.UserConstructionScript`))