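; Base actor for "add ability" powerup upgrades that grant a gameplay ability to the player.
; One tick after BeginPlay, it gives AbilityToGrant to player character 0's Ability System Component through GiveAbilityAndActivateOnce, then destroys itself.
; The actor is a fire-and-forget applier with no active overlap or tick logic, so spawning it is what applies the upgrade.
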(event `self.ReceiveBeginPlay`
  (`parent.ReceiveBeginPlay`)
  (`KismetSystemLibrary.DelayUntilNextTick`)
  (`self.ApplyUpgrade`))

(event `self.ApplyUpgrade`
  (`AbilitySystemComponent.K2_GiveAbilityAndActivateOnce` (`AbilitySystemBlueprintLibrary.GetAbilitySystemComponent` (`GameplayStatics.GetPlayerCharacter` 0)) (`self.AbilityToGrant`) 0 -1)
  (`self.K2_DestroyActor`))

(fn `UserConstructionScript`
  (`parent.UserConstructionScript`))