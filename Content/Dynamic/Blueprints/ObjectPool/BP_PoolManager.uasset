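; Object pool manager that pre-spawns ranged enemies and reuses them on request.
; On BeginPlay it spawns MaxEnemiesCount BP_EnemyRanged_Base actors at the world origin into EnemiesPool.
; SpawnEnemyFromPool uses a linear search for an enemy not in use, then marks it in use with the given transform through SetIsInUse.
; The search prints a message when it finds no valid enemy; the pool never grows.
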(event `self.ReceiveBeginPlay`
  (`self.SpawnEnemies`))

(event `SpawnEnemies`
  (for _ (range (`self.MaxEnemiesCount`))
    (bind _returnvalue (`|SpawnActorFromClass` "/Game/Dynamic/Blueprints/Controllers/Enemies/EnemyBase/BP_EnemyRanged_Base.BP_EnemyRanged_Base_C" (`KismetMathLibrary.MakeTransform` (0.0 0.0 0.0)) "Undefined" "MultiplyWithRoot" null null))
    (`KismetArrayLibrary.Array_AddUnique` (`self.EnemiesPool`) _returnvalue)))

(fn `FindFisrtAvailableEnemy`
  (returns (Enemy :type "/Game/Dynamic/Blueprints/Controllers/Enemies/EnemyBase/BP_Enemy_Base Object Reference"))
  (locals (AvailableEnemy :type "/Game/Dynamic/Blueprints/Controllers/Enemies/EnemyBase/BP_Enemy_Base Object Reference"))
  (for _array_element (`self.EnemiesPool`)
    (if (not (`/Game/Dynamic/Blueprints/Controllers/Enemies/EnemyBase/BP_Enemy_Base.IsInUse?` _array_element))
      (set `local.AvailableEnemy` _array_element)
      (break)))
  (bind _availableenemy (`local.AvailableEnemy`)
    (:`then`
      (return _availableenemy))
    (:`else`
      (`KismetSystemLibrary.PrintString` "NO AVAILABLE ENEMY"))))

(fn `SpawnEnemyFromPool`
  (params (EnemySpawnTransform :type "Transform Structure"))
  (bind _enemy (`self.FindFisrtAvailableEnemy`))
  (`/Engine/EditorBlueprintResources/StandardMacros.IsValid` _enemy
    (:`Is Valid`
      (`/Game/Dynamic/Blueprints/Controllers/Enemies/EnemyBase/BP_Enemy_Base.SetIsInUse` _enemy true EnemySpawnTransform))))

(fn `UserConstructionScript`)