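; Enemy object pool manager that pre-spawns inactive enemies for each class in its pool map on BeginPlay, then tells GM_Prototype to begin the game.
; SpawnEnemyFromPool and SpawnBoss activate the first unused pooled actor through SetIsInUse, printing a warning if none is free.
; Spawn locations are randomly offset from the player, with independent X and Y angles, and SpawnEnemyFromPool ignores its transform input.
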(event `self.ReceiveBeginPlay`
  (`self.SpawnEnemies`))

(event `SpawnEnemies`
  (bind _enemypoolsmap (`self.EnemyPoolsMap`))
  (bind (_keypin _valuepin) (`|MapForEach` _enemypoolsmap)
    (:`then`
      (`KismetArrayLibrary.Array_Clear` (`self.TemporaryEnemyPool`))
      (bind (_poolarray _initialcount _isinitialized) (break `/Game/Dynamic/Blueprints/ObjectPool/Enemy/Str_EnemyPoolData` _valuepin))
      (if (not _isinitialized)
        (for _ (range _initialcount)
          (bind _returnvalue (`|SpawnActorFromClass` _keypin (`KismetMathLibrary.MakeTransform` (0.0 0.0 0.0)) "Undefined" "MultiplyWithRoot" null (`BlueprintMapLibrary.Map_Find` (`self.EnemyDefaultStatsForClass`) _keypin) null))
          (`KismetArrayLibrary.Array_AddUnique` (`self.TemporaryEnemyPool`) _returnvalue)
          (`/Game/Dynamic/Blueprints/Controllers/Enemies/EnemyBase/BP_Enemy_Base.SetIsInUse` :`self` _returnvalue))
        (`BlueprintMapLibrary.Map_Add` _enemypoolsmap _keypin (make `/Game/Dynamic/Blueprints/ObjectPool/Enemy/Str_EnemyPoolData` (`self.TemporaryEnemyPool`) _initialcount true))))
    (:`CompletedPin`
      (bind _asgm_prototype (cast `/Game/Dynamic/Blueprints/Controllers/GM_Prototype` (`GameplayStatics.GetGameMode`)))
      (`/Game/Dynamic/Blueprints/Controllers/GM_Prototype.BeginGame` _asgm_prototype))))

(fn `FindFisrtAvailableEnemy`
  (params (EnemiesPool :type "Array of /Game/Dynamic/Blueprints/Controllers/Enemies/EnemyBase/BP_Enemy_Base Object Reference"))
  (returns (Enemy :type "/Game/Dynamic/Blueprints/Controllers/Enemies/EnemyBase/BP_Enemy_Base Object Reference"))
  (locals (AvailableEnemy :type "/Game/Dynamic/Blueprints/Controllers/Enemies/EnemyBase/BP_Enemy_Base Object Reference"))
  (for _array_element EnemiesPool
    (if (not (`/Game/Dynamic/Blueprints/Controllers/Enemies/EnemyBase/BP_Enemy_Base.IsInUse?` _array_element))
      (set `local.AvailableEnemy` _array_element)
      (break)))
  (bind _availableenemy (`local.AvailableEnemy`)
    (:`then`
      (return _availableenemy))
    (:`else`
      (`KismetSystemLibrary.PrintString` "NO AVAILABLE ENEMY"))))

(fn `FindPoolForEnemies`
  (params (EnemyClass :type "/Game/Dynamic/Blueprints/Controllers/Enemies/EnemyBase/BP_Enemy_Base Class Reference"))
  (returns (Pool :type "Array of /Game/Dynamic/Blueprints/Controllers/Enemies/EnemyBase/BP_Enemy_Base Object Reference"))
  (return (`.PoolArray_3_FC877BA1481914950243E4988773CF83` (break `/Game/Dynamic/Blueprints/ObjectPool/Enemy/Str_EnemyPoolData` (`BlueprintMapLibrary.Map_Find` (`self.EnemyPoolsMap`) EnemyClass)))))

(fn `GetEnemySpawnTransform`
  (params (SpawnRadius :type "Float (double-precision)"))
  (returns (SpawnTransform :type "Transform Structure"))
  (bind _returnvalue (`KismetMathLibrary.RandomFloatInRange` 0.0 360.0))
  (bind (_returnvalue_location _returnvalue_rotation _returnvalue_scale) (`KismetMathLibrary.BreakTransform` (`self.GetTransform` (`GameplayStatics.GetPlayerCharacter` 0))))
  (return (`KismetMathLibrary.MakeTransform` (+ _returnvalue_location (`KismetMathLibrary.MakeVector` (* (`KismetMathLibrary.DegCos` _returnvalue) SpawnRadius) (* (`KismetMathLibrary.DegSin` _returnvalue) SpawnRadius))) _returnvalue_rotation _returnvalue_scale)))

(fn `SpawnBoss`
  (returns (Boss :type "/Game/Dynamic/Blueprints/Controllers/Enemies/EnemyBase/BP_Enemy_Base Object Reference"))
  (bind _enemy (`self.FindFisrtAvailableEnemy` (`.PoolArray_3_FC877BA1481914950243E4988773CF83` (break `/Game/Dynamic/Blueprints/ObjectPool/Enemy/Str_EnemyPoolData` (`BlueprintMapLibrary.Map_Find` (`self.EnemyPoolsMap`) "/Game/Dynamic/Blueprints/Controllers/Enemies/EnemyBase/Boss/BP_Boss.BP_Boss_C")))))
  (`/Engine/EditorBlueprintResources/StandardMacros.IsValid` _enemy
    (:`Is Valid`
      (`/Game/Dynamic/Blueprints/Controllers/Enemies/EnemyBase/BP_Enemy_Base.SetIsInUse` _enemy true (`self.GetEnemySpawnTransform` 200.0))
      (`KismetSystemLibrary.PrintString` (`KismetSystemLibrary.GetDisplayName` _enemy))
      (return _enemy))))

(fn `SpawnEnemyFromPool`
  (params (EnemySpawnTransform :type "Transform Structure") (EnemyClass :type "/Game/Dynamic/Blueprints/Controllers/Enemies/EnemyBase/BP_Enemy_Base Class Reference"))
  (bind _enemy (`self.FindFisrtAvailableEnemy` (`self.FindPoolForEnemies` EnemyClass)))
  (`/Engine/EditorBlueprintResources/StandardMacros.IsValid` _enemy
    (:`Is Valid`
      (`/Game/Dynamic/Blueprints/Controllers/Enemies/EnemyBase/BP_Enemy_Base.SetIsInUse` _enemy true (`self.GetEnemySpawnTransform` (`self.BaseEnemySpawnRadius`))))))

(fn `UserConstructionScript`)