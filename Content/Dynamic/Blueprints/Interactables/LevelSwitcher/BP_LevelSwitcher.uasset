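; BP_LevelSwitcher is an interactable that offers the player a switch from the lobby to a run level.
; Entering its sphere caches the BP_Player and shows a Press F prompt widget, which is removed on exit.
; Interact opens a WBP_SwitchLobbyToRunLevel widget passed LevelToSwitch, switches input to UI only with a visible cursor, stops the player's movement and pauses the game.
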(event `/Game/Dynamic/Blueprints/InteractibleSystem/Interfaces/BPI_Interaction.Interact`
  (bind _returnvalue (`GameplayStatics.GetPlayerController` 0))
  (bind _returnvalue_2 (`|CreateWidget` "/Game/Dynamic/Blueprints/WidgetBlueprint(WBP)/Menus/SwitchLevels/SwitchLobbyToRunLevelMenu/WBP_SwitchLobbyToRunLevel.WBP_SwitchLobbyToRunLevel_C" null (`self.LevelToSwitch`)))
  (`UserWidget.AddToViewport` _returnvalue_2 0)
  (`WidgetBlueprintLibrary.SetInputMode_UIOnlyEx` _returnvalue _returnvalue_2)
  (set `PlayerController.bShowMouseCursor` true _returnvalue)
  (`MovementComponent.StopMovementImmediately` (`Character.CharacterMovement` (`self.PlayerRef`)))
  (`GameplayStatics.SetGamePaused` true))

(event `self.Sphere.OnComponentBeginOverlap`
  (params (OverlappedComponent :type "PrimitiveComponent Object Reference") (OtherActor :type "Actor Object Reference") (OtherComp :type "PrimitiveComponent Object Reference") (OtherBodyIndex :type Integer) (bFromSweep :type Boolean) (SweepResult :type "HitResult Structure (by ref)"))
  (bind _asbp_player (cast `/Game/Dynamic/Blueprints/Controllers/Player/BP_Player` OtherActor))
  (set `self.PlayerRef` _asbp_player)
  (bind _returnvalue (`|CreateWidget` "/Game/Dynamic/Blueprints/WidgetBlueprint(WBP)/Prototype/WBP_PressF.WBP_PressF_C"))
  (bind _output_get (set `self.FWidget` _returnvalue))
  (`UserWidget.AddToViewport` _output_get 0))

(event `self.Sphere.OnComponentEndOverlap`
  (params (OverlappedComponent :type "PrimitiveComponent Object Reference") (OtherActor :type "Actor Object Reference") (OtherComp :type "PrimitiveComponent Object Reference") (OtherBodyIndex :type Integer))
  (cast `/Game/Dynamic/Blueprints/Controllers/Player/BP_Player` OtherActor)
  (`Widget.RemoveFromParent` (`self.FWidget`)))

(fn `UserConstructionScript`)