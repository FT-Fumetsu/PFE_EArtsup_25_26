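; Chest pickup that offers the player a choice of power-ups, drawn from a data table, when they overlap it.
; It picks distinct rows by rarity-weighted random selection, removing each winner from the pool until the choice count is reached.
; The chest then destroys itself, pauses the game and shows WBP_Chest with the choices in UI-only input.
; ApplyPowerUp is an empty stub.
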(event `self.Collider.OnComponentBeginOverlap`
  (params (OverlappedComponent :type "PrimitiveComponent Object Reference") (OtherActor :type "Actor Object Reference") (OtherComp :type "PrimitiveComponent Object Reference") (OtherBodyIndex :type Integer) (bFromSweep :type Boolean) (SweepResult :type "HitResult Structure (by ref)"))
  (bind _returnvalue (`GameplayStatics.GetPlayerController` 0))
  (cast `/Game/Dynamic/Blueprints/Controllers/Player/BP_Player` OtherActor)
  (if (not (`self.IsOpen`))
    (set `self.IsOpen` true)
    (set `self.PlayerRef` (`GameplayStatics.GetPlayerCharacter` 0))
    (`KismetArrayLibrary.Array_Clear` (`self.RowPool`))
    (`KismetArrayLibrary.Array_Clear` (`self.SelectedRowStructs`))
    (bind _outrownames (`DataTableFunctionLibrary.GetDataTableRowNames` (`self.DataTable`)))
    (for _array_element _outrownames
      (`KismetArrayLibrary.Array_AddUnique` (`self.RowPool`) _array_element))
    (while (and (< (`KismetArrayLibrary.Array_Length` (`self.SelectedRowStructs`)) (`self.ChoiceCount`)) (`KismetArrayLibrary.Array_IsNotEmpty` (`self.RowPool`)))
      (set `self.TotalWeight` 0)
      (for _array_element_2 (`self.RowPool`)
        (bind _returnvalue_2 (`|GetDataTableRow` (`self.DataTable`) _array_element_2)
          (:`then`
            (`self.GetWeightForRarity` (`.Rarity_20_C33BCB9F400591889A4ECCB9557C33BB` (break `/Game/Dynamic/Blueprints/Structures/PowerUps/Str_PowerUps` _returnvalue_2)))
            (set `self.TotalWeight` (+ (`self.TotalWeight`) (`self.CurrentWeight`))))))
      (set `self.RandomWeight` (`KismetMathLibrary.RandomIntegerInRange` 0 (`self.TotalWeight`)))
      (for _array_element_3 (`self.RowPool`)
        (bind _returnvalue_3 (`|GetDataTableRow` (`self.DataTable`) _array_element_3)
          (:`then`
            (`self.GetWeightForRarity` (`.Rarity_20_C33BCB9F400591889A4ECCB9557C33BB` (break `/Game/Dynamic/Blueprints/Structures/PowerUps/Str_PowerUps` _returnvalue_3)))
            (bind _output_get (set `self.Cumulative` (+ (`self.Cumulative`) (`self.CurrentWeight`))))
            (if (>= _output_get (`self.RandomWeight`))
              (`KismetArrayLibrary.Array_AddUnique` (`self.SelectedRowStructs`) _returnvalue_3)
              (`KismetArrayLibrary.Array_RemoveItem` (`self.RowPool`) _array_element_3)
              (set `self.Cumulative` 0)
              (break))))))
    (`self.K2_DestroyActor`)
    (bind _returnvalue_4 (`|CreateWidget` "/Game/Dynamic/Blueprints/WidgetBlueprint(WBP)/Chests/WBP_Chest.WBP_Chest_C"))
    (`UserWidget.AddToViewport` _returnvalue_4 0)
    (set `PlayerController.bShowMouseCursor` true _returnvalue)
    (`WidgetBlueprintLibrary.SetInputMode_UIOnlyEx` _returnvalue null)
    (`MovementComponent.StopMovementImmediately` (`Character.CharacterMovement` (cast `/Game/Dynamic/Blueprints/Controllers/Player/BP_Player` (`self.PlayerRef`) :!pure true)))
    (`GameplayStatics.SetGamePaused` true)
    (`/Game/Dynamic/Blueprints/WidgetBlueprint(WBP)/Chests/WBP_Chest.InitializeCoices` _returnvalue_4 (`self.SelectedRowStructs`))
    (add `/Game/Dynamic/Blueprints/WidgetBlueprint(WBP)/Chests/WBP_Chest.OnChoiceClicked` _returnvalue_4 (`|CreateDelegate` :!event `ApplyPowerUp`))))

(event `GetWeightForRarity`
  (params (Rarity :type "/Game/Dynamic/Blueprints/Enums/PowerUps/E_PowerUpsRarity Enum" :default "NewEnumerator0"))
  (switch `/Game/Dynamic/Blueprints/Enums/PowerUps/E_PowerUpsRarity` Rarity
    (:`NewEnumerator0`
      (set `self.CurrentWeight` 30))
    (:`NewEnumerator1`
      (set `self.CurrentWeight` 15))
    (:`NewEnumerator2`
      (set `self.CurrentWeight` 10))
    (:`NewEnumerator3`
      (set `self.CurrentWeight` 6))
    (:`NewEnumerator4`
      (set `self.CurrentWeight` 3))
    (:`NewEnumerator5`
      (set `self.CurrentWeight` 1))))

(event `ApplyPowerUp`
  (params (RowPowerUp :type "/Game/Dynamic/Blueprints/Structures/PowerUps/Str_PowerUps Structure")))

(fn `UserConstructionScript`)