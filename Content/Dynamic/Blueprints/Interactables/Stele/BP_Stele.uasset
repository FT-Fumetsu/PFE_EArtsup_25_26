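; BP_Stele is an interactable stele that offers the player a choice of upgrades after they stay inside its interaction area for a set time.
; Overlap events track the player, Tick accumulates dwell time up to the cooldown, and leaving resets the timer.
; On activation it finds the BP_PowerupChoiceManager in the level, passes its upgrade array and choice count to ChooseUpgrades, then disables its tick, making it single-use.
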(event `self.ReceiveTick`
  (params (DeltaSeconds :type "Float (single-precision)"))
  (if (and (`self.IsPlayerInRadius`) (not (`self.IsActivated`)))
    (set `self.ElapsedTime` (+ DeltaSeconds (`self.ElapsedTime`)))
    (if (>= (`self.ElapsedTime`) (`self.InteractionCooldown`))
      (`self.Interact`))))

(event `Interact`
  (set `self.IsActivated` true)
  (bind _returnvalue (`GameplayStatics.GetActorOfClass` "/Game/Dynamic/Blueprints/Powerups/BP_PowerupChoiceManager.BP_PowerupChoiceManager_C"))
  (`/Engine/EditorBlueprintResources/StandardMacros.IsValid` _returnvalue
    (:`Is Valid`
      (`/Game/Dynamic/Blueprints/Powerups/BP_PowerupChoiceManager.ChooseUpgrades` _returnvalue (`self.UpgradeArray`) (`self.ChoiceCount`))
      (`self.SetActorTickEnabled` false))
    (:`Is Not Valid`
      (`KismetSystemLibrary.PrintString` "Stèle : Powerup Choice Manager == null"))))

(event `self.InteractionArea.OnComponentBeginOverlap`
  (params (OverlappedComponent :type "PrimitiveComponent Object Reference") (OtherActor :type "Actor Object Reference") (OtherComp :type "PrimitiveComponent Object Reference") (OtherBodyIndex :type Integer) (bFromSweep :type Boolean) (SweepResult :type "HitResult Structure (by ref)"))
  (if (== OtherActor (`GameplayStatics.GetPlayerCharacter` 0))
    (set `self.IsPlayerInRadius` true)))

(event `self.InteractionArea.OnComponentEndOverlap`
  (params (OverlappedComponent :type "PrimitiveComponent Object Reference") (OtherActor :type "Actor Object Reference") (OtherComp :type "PrimitiveComponent Object Reference") (OtherBodyIndex :type Integer))
  (if (== OtherActor (`GameplayStatics.GetPlayerCharacter` 0))
    (set `self.IsPlayerInRadius` false)
    (set `self.ElapsedTime` 0.0)))

(fn `UserConstructionScript`)