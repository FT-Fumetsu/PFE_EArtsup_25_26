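; Prototype game mode that starts a play session when its BeginGame event is called.
; It spawns BP_Player at a random PlayerStart, passes it StartingAbility as a debug ability grant, and possesses it with the first player controller.
; If that controller is a PC_BaseController, it notifies it of game begin, enables game state ticking, and tells BP_GameFlowManager to begin spawns.
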(event `BeginGame`
  (bind _outactors (`GameplayStatics.GetAllActorsOfClass` "/Script/Engine.PlayerStart"))
  (bind _returnvalue (`|SpawnActorFromClass` "/Game/Dynamic/Blueprints/Controllers/Player/BP_Player.BP_Player_C" (`self.GetTransform` (`KismetArrayLibrary.Array_Random` _outactors)) "Undefined" "MultiplyWithRoot" null "/Game/Static/DefaultUE5Characters/Mannequins/Anims/Unarmed/Attack/AM_Attack_01.AM_Attack_01" 0.3 600.0 (struct) null))
  (set `/Game/Dynamic/Blueprints/Controllers/Player/BP_Player.DebugAbilityToGrantAtStart` (`self.StartingAbility`) _returnvalue)
  (`Controller.Possess` (`GameplayStatics.GetPlayerController` 0) _returnvalue)
  (bind _aspc_base_controller (cast `/Game/Dynamic/Blueprints/Controllers/Player/PC_BaseController` (`GameplayStatics.GetPlayerController` 0)))
  (`/Game/Dynamic/Blueprints/Controllers/Player/PC_BaseController.OnGameBegin` _aspc_base_controller)
  (`self.SetActorTickEnabled` (`GameplayStatics.GetGameState`) true)
  (bind _returnvalue_2 (`GameplayStatics.GetActorOfClass` "/Game/Dynamic/Blueprints/WaveSystem/BP_GameFlowManager.BP_GameFlowManager_C"))
  (`/Game/Dynamic/Blueprints/WaveSystem/BP_GameFlowManager.BeginSpawns` _returnvalue_2))

(fn `UserConstructionScript`)