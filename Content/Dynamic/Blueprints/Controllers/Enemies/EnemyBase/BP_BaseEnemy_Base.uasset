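; Base enemy character that chases the player and attacks on reaching attack range.
; Each tick it checks the player's ability system for the State.Dead tag, stopping its movement if present and otherwise issuing AIMoveTo with AttackDistance as acceptance radius.
; A successful move calls Attack, gated by a CanAttack flag that is cleared first and not reset in this graph.
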(event `self.ReceiveTick`
  (params (DeltaSeconds :type "Float (single-precision)"))
  (if (not (`GameplayTagAssetInterface.HasMatchingGameplayTag` (`AbilitySystemBlueprintLibrary.GetAbilitySystemComponent` (`GameplayStatics.GetPlayerCharacter` 0)) (struct :`TagName` "State.Dead")))
    (`|AIMoveTo` self (0.0 0.0 0.0) (`GameplayStatics.GetPlayerCharacter` 0) (`self.AttackDistance`)
      (:`OnSuccess`
        (if (`self.canAttack?`)
          (set `self.canAttack?` false)
          (`self.Attack`))))
    (else
      (`MovementComponent.StopMovementImmediately` (`self.CharacterMovement`)))))

(fn `UserConstructionScript`
  (`parent.UserConstructionScript`))