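; Test enemy character that chases the player and makes GAS gauntlet melee attacks on reaching them.
; An attribute change triggers a delayed gauntlet equip event and walk speed setting, while Tick drives movement and attacks.
; SetIsInUse supports pool-style reuse, toggling visibility, tick, collision and gravity, resetting health on activation and deactivating shortly after death.
; Health, healing and damage calls delegate to ACDamageSystem.
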(event `self.ReceiveBeginPlay`
  (`AbilityAsync_WaitAttributeChanged.WaitForAttributeChanged` null (struct :`AttributeName` "Health" :`Attribute` "/Script/PFE_EArtsup_25_26.BasicAttributeSet:Health" :`AttributeOwner` "/Script/CoreUObject.Class'/Script/PFE_EArtsup_25_26.BasicAttributeSet'")
    (:`then`
      (`KismetSystemLibrary.Delay` 0.2)
      (`AbilitySystemBlueprintLibrary.SendGameplayEventToActor` self (struct :`TagName` "Event.Weapon.Equip") (make `GameplayEventData` :`TargetTags` (struct :`GameplayTags` (struct :`(TagName` "Weapon.Melee.Gauntelts")))))
      (set `CharacterMovementComponent.MaxWalkSpeed` 300.0 (`self.CharacterMovement`)))))

(event `self.ReceiveTick`
  (params (DeltaSeconds :type "Float (single-precision)"))
  (`|AIMoveTo` self (0.0 0.0 0.0) (`GameplayStatics.GetPlayerCharacter` 0) (`self.MoveToPlayerAcceptanceRadius`)
    (:`OnSuccess`
      (if (`self.canAttack?`)
        (set `self.canAttack?` false)
        (`self.Attack`)))))

(event `Attack`
  (`AbilitySystemComponent.TryActivateAbilityByClass` (`self.AbilitySystemComponent`) "/Game/Dynamic/Blueprints/GameplayAbilitySystem/Abilities/Attacks/GA_MeleeAttack_Gauntlets.GA_MeleeAttack_Gauntlets_C" true)
  (set `self.canAttack?` true))

(event `self.HandleDeath`
  (`parent.HandleDeath`)
  (`KismetSystemLibrary.Delay` 1.0)
  (`self.SetIsInUse` false))

(fn `GetCurrentHealth`
  (returns (Health :type "Float (double-precision)"))
  (return (`/Game/Dynamic/Blueprints/DamageSystem/ActorComponents/AC_DamageSystem.Health` (`self.AC_DamageSystem`))))

(fn `GetMaxHealth`
  (returns (MaxHealth :type "Float (double-precision)"))
  (return (`/Game/Dynamic/Blueprints/DamageSystem/ActorComponents/AC_DamageSystem.MaxHealth` (`self.AC_DamageSystem`))))

(fn `Heal`
  (params (Amount :type "Float (double-precision)"))
  (returns (NewHealth :type "Float (double-precision)"))
  (bind _newhealth (`/Game/Dynamic/Blueprints/DamageSystem/ActorComponents/AC_DamageSystem.Heal` (`self.AC_DamageSystem`) Amount))
  (return _newhealth))

(fn `SetIsInUse`
  (params (`IsInUse?` :type Boolean) (SpawnTransform :type "Transform Structure"))
  (locals (BaseTransform :type "Transform Structure" :default "0.000000,0.000000,-2000.000000|0.000000,0.000000,0.000000|1.000000,1.000000,1.000000"))
  (bind _ac_damagesystem (`self.AC_DamageSystem`))
  (bind _output_get (set `self.IsInUse?` `IsInUse?`))
  (`self.SetActorHiddenInGame` (not _output_get))
  (`self.SetActorTickEnabled` _output_get)
  (`self.SetActorEnableCollision` _output_get)
  (set `CharacterMovementComponent.GravityScale` (`KismetMathLibrary.SelectFloat` 1.0 0.0 _output_get) (`self.CharacterMovement`))
  (if _output_get
    (set `/Game/Dynamic/Blueprints/DamageSystem/ActorComponents/AC_DamageSystem.Health` (`/Game/Dynamic/Blueprints/DamageSystem/ActorComponents/AC_DamageSystem.MaxHealth` _ac_damagesystem) _ac_damagesystem)
    (set `/Game/Dynamic/Blueprints/DamageSystem/ActorComponents/AC_DamageSystem.IsDead?` false _ac_damagesystem)
    (`self.K2_SetActorTransform` (`local.SpawnTransform`))
    (else
      (`self.K2_SetActorTransform` (`local.BaseTransform`)))))

(fn `TakeDamage`
  (params (DamageInfo :type "/Game/Dynamic/Blueprints/DamageSystem/Structures/Str_DamageInfo Structure"))
  (returns (`WasDamaged?` :type Boolean))
  (bind _wasdamaged_ (`/Game/Dynamic/Blueprints/DamageSystem/ActorComponents/AC_DamageSystem.TakeDamage` (`self.AC_DamageSystem`) DamageInfo))
  (return _wasdamaged_))

(fn `UserConstructionScript`
  (`self.SetIsInUse` false))