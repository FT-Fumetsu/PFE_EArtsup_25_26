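; Base enemy character on the Gameplay Ability System that chases the player and attacks on arrival.
; Tick runs AIMoveTo until the player is dead, while Attack and the range and target getters are empty stubs, apparently for child overrides.
; BeginPlay equips melee gauntlets via gameplay event and sets walk speed.
; SetIsInUse supports pooling by toggling visibility, tick, collision and gravity; death spawns XP coins, then deactivates the enemy.
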(event `self.ReceiveBeginPlay`
  (`AbilityAsync_WaitAttributeChanged.WaitForAttributeChanged` null (struct :`AttributeName` "Health" :`Attribute` "/Script/PFE_EArtsup_25_26.BasicAttributeSet:Health" :`AttributeOwner` "/Script/CoreUObject.Class'/Script/PFE_EArtsup_25_26.BasicAttributeSet'")
    (:`then`
      (`KismetSystemLibrary.Delay` 0.2)
      (`AbilitySystemBlueprintLibrary.SendGameplayEventToActor` self (struct :`TagName` "Event.Weapon.Equip") (make `GameplayEventData` :`TargetTags` (struct :`GameplayTags` (struct :`(TagName` "Weapon.Melee.Gauntelts")))))
      (set `CharacterMovementComponent.MaxWalkSpeed` 300.0 (`self.CharacterMovement`)))))

(event `self.ReceiveTick`
  (params (DeltaSeconds :type "Float (single-precision)"))
  (if (not (`GameplayTagAssetInterface.HasMatchingGameplayTag` (`AbilitySystemBlueprintLibrary.GetAbilitySystemComponent` (`GameplayStatics.GetPlayerCharacter` 0)) (struct :`TagName` "State.Dead")))
    (`|AIMoveTo` self (0.0 0.0 0.0) (`GameplayStatics.GetPlayerCharacter` 0) (`self.MoveToPlayerAcceptanceRadius`)
      (:`OnSuccess`
        (if (`self.canAttack?`)
          (set `self.canAttack?` false)
          (`self.Attack`))))
    (else
      (`MovementComponent.StopMovementImmediately` (`self.CharacterMovement`)))))

(event `self.HandleDeath`
  (`parent.HandleDeath`)
  (for _ (range (`self.ExperiencePiecesNumber`))
    (`|SpawnActorFromClass` "/Game/Dynamic/Blueprints/Experience/BP_XPCoin.BP_XPCoin_C" (`self.GetTransform`) "Undefined" "MultiplyWithRoot" null null))
  (`KismetSystemLibrary.Delay` 1.0)
  (`self.SetIsInUse` false))

(fn `Attack`)

(fn `GetAttackRange`
  (returns (AttackRange :type "Float (double-precision)"))
  (return 0.0))

(fn `GetAttackTarget`
  (params (MaxSearchingRange :type "Float (double-precision)") (`Projectile?` :type Boolean))
  (returns (AttackTarget :type "Actor Object Reference"))
  (return null))

(fn `GetProjectileRange`
  (returns (ProjectileRange :type "Float (double-precision)"))
  (return 0.0))

(fn `SetIsInUse`
  (params (`IsInUse?` :type Boolean) (SpawnTransform :type "Transform Structure"))
  (locals (BaseTransform :type "Transform Structure" :default "0.000000,0.000000,-2000.000000|0.000000,0.000000,0.000000|1.000000,1.000000,1.000000"))
  (bind _output_get (set `self.IsInUse?` `IsInUse?`))
  (`self.SetActorHiddenInGame` (not _output_get))
  (`self.SetActorTickEnabled` _output_get)
  (`self.SetActorEnableCollision` _output_get)
  (set `CharacterMovementComponent.GravityScale` (`KismetMathLibrary.SelectFloat` 1.0 0.0 _output_get) (`self.CharacterMovement`))
  (if _output_get
    (`self.K2_SetActorTransform` (`local.SpawnTransform`))
    (else
      (`self.K2_SetActorTransform` (`local.BaseTransform`)))))

(fn `UserConstructionScript`
  (`self.SetIsInUse` false))