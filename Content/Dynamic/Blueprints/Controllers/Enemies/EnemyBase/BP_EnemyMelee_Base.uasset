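; Base melee enemy Blueprint that attacks the player through the Gameplay Ability System.
; Its Attack override calls the parent, then TryToAttack sets AI focus on the target, activates the AttackToUse ability and restores CanAttack after a Cooldown delay.
; GetAttackTarget always returns the first player character, ignoring its range and projectile inputs, and GetAttackRange returns AttackDistance.
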(event `self.ReceiveTick`
  (params (DeltaSeconds :type "Float (single-precision)"))
  (`parent.ReceiveTick` DeltaSeconds))

(event `TryToAttack`
  (bind _attacktarget (`/Game/Dynamic/Blueprints/GameplayAbilitySystem/Interfaces/BPI_Targetting.GetAttackTarget` 0.0))
  (`AIController.K2_SetFocus` (`AIBlueprintHelperLibrary.GetAIController` self) _attacktarget)
  (`AbilitySystemComponent.TryActivateAbilityByClass` (`self.AbilitySystemComponent`) (`self.AttackToUse`) true)
  (`KismetSystemLibrary.Delay` (`self.Cooldown`))
  (set `self.canAttack?` true))

(fn `Attack`
  (`parent.Attack`)
  (`self.TryToAttack`))

(fn `GetAttackRange`
  (returns (AttackRange :type "Float (double-precision)"))
  (return (`self.AttackDistance`)))

(fn `GetAttackTarget`
  (params (MaxSearchingRange :type "Float (double-precision)") (`Projectile?` :type Boolean))
  (returns (AttackTarget :type "Actor Object Reference"))
  (return (`GameplayStatics.GetPlayerCharacter` 0)))

(fn `UserConstructionScript`
  (`parent.UserConstructionScript`))