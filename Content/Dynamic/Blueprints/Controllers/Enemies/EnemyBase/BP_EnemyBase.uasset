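; Base enemy character that chases the player and plays an attack montage once it gets within reach.
; Every Tick issues an AIMoveTo toward player 0 using a configurable acceptance radius.
; On success, a CanAttack flag gates the montage and is restored after a delay matching its returned length.
; Tick also sets CanAttack to true every frame, so the gate does not hold between frames.
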(event `self.ReceiveTick`
  (params (DeltaSeconds :type "Float (single-precision)"))
  (set `self.canAttack?` true)
  (`|AIMoveTo` self (0.0 0.0 0.0) (`GameplayStatics.GetPlayerCharacter` 0) (`self.MoveToPlayerAcceptanceRadius`)
    (:`OnSuccess`
      (if (`self.canAttack?`)
        (set `self.canAttack?` false)
        (bind _returnvalue (`self.PlayAnimMontage` (`self.EnemyAttackMontage`)))
        (`KismetSystemLibrary.Delay` _returnvalue)
        (set `self.canAttack?` true)))))

(fn `UserConstructionScript`)