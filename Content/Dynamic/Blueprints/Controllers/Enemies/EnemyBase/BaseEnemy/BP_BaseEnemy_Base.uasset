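; Base enemy Blueprint that chases the first player character and attacks within AttackDistance.
; SetIsInUse calls the parent, then starts FollowPlayer when the enemy is activated.
; FollowPlayer attacks if in range and CanAttack is set, clearing that flag first, otherwise runs AIMoveTo, attacking on success and retrying immediately on failure.
; GetAttackRange and GetAttackTarget are empty stubs, and the next-tick retry delay is unconnected.
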(event `FollowPlayer`
  (bind _returnvalue (`GameplayStatics.GetPlayerCharacter` 0))
  (bind _attackdistance (`self.AttackDistance`))
  (if (and (`self.IsInUse?`) (not (`self.IsDead`)))
    (`/Engine/EditorBlueprintResources/StandardMacros.IsValid` _returnvalue
      (:`Is Valid`
        (if (<= (`KismetMathLibrary.Vector_Distance` (`self.K2_GetActorLocation`) (`self.K2_GetActorLocation` _returnvalue)) _attackdistance)
          (if (`self.canAttack?`) :!label _label
            (set `self.canAttack?` false)
            (`self.Attack`))
          (else
            (`|AIMoveTo` self (0.0 0.0 0.0) _returnvalue _attackdistance
              (:`OnSuccess`
                (goto _label))
              (:`OnFail`
                (`self.FollowPlayer`)))))))))

(fn `GetAttackRange`
  (returns (AttackRange :type "Float (double-precision)"))
  (return 0.0))

(fn `GetAttackTarget`
  (params (MaxSearchingRange :type "Float (double-precision)") (`Projectile?` :type Boolean) (EnemiesArray :type "Array of /Game/Dynamic/Blueprints/Controllers/Enemies/EnemyBase/BP_Enemy_Base Object Reference (by ref)") (ActorsToIgnore :type "Array of Actor Object Reference (by ref)"))
  (returns (AttackTarget :type "Actor Object Reference"))
  (return null))

(fn `SetIsInUse`
  (params (`IsInUse?` :type Boolean) (SpawnTransform :type "Transform Structure") (`IsRespawned?` :type Boolean))
  (`parent.SetIsInUse` `IsInUse?` SpawnTransform `IsRespawned?`)
  (if `IsInUse?`
    (`self.FollowPlayer`)))

(fn `UserConstructionScript`
  (`parent.UserConstructionScript`))