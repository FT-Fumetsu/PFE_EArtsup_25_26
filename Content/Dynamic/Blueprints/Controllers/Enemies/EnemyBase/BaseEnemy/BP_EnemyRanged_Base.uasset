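; Base ranged enemy that attacks the player with a projectile through the Gameplay Ability System, using Changelin attack and hit-reaction montages.
; Attacking plays the montage and waits for its shoot gameplay event, then line-traces to confirm the player is visible.
; On a clear shot it focuses the player, activates the projectile ability, and re-enables attacking after a cooldown.
; It resumes following the player after that cooldown or when the montage ends.
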(event `self.ReceiveTick`
  (params (DeltaSeconds :type "Float (single-precision)"))
  (`parent.ReceiveTick` DeltaSeconds))

(event `TryToAttack`
  (if (not (`self.IsDead`))
    (`|PlayMontage` (`self.Mesh`) "/Game/Static/08_Characters/Changelin/AM_Changelin_Attack.AM_Changelin_Attack"
      (:`then`
        (`AbilityAsync_WaitGameplayEvent.WaitGameplayEventToActor` null (struct :`TagName` "Event.ShootProjectile") true
          (:`EventReceived`
            (bind _attacktarget (`/Game/Dynamic/Blueprints/GameplayAbilitySystem/Interfaces/BPI_Targetting.GetAttackTarget` 0.0))
            (`/Engine/EditorBlueprintResources/StandardMacros.IsValid` _attacktarget
              (:`Is Valid`
                (`AIController.K2_SetFocus` (`AIBlueprintHelperLibrary.GetAIController` self) _attacktarget)
                (`AbilitySystemComponent.TryActivateAbilityByClass` (`self.AbilitySystemComponent`) "/Game/Dynamic/Blueprints/GameplayAbilitySystem/Abilities/Attacks/EnemiesAttacks/GA_EnemyShootProjectile_Base.GA_EnemyShootProjectile_Base_C" true)
                (`KismetSystemLibrary.Delay` (`self.Cooldown`))
                (set `self.canAttack?` true)
                (`self.FollowPlayer`))))))
      (:`OnCompleted`
        (`self.FollowPlayer` :!label _label))
      (:`OnInterrupted`
        (goto _label)))))

(fn `Attack`
  (`parent.Attack`)
  (`self.TryToAttack`))

(fn `GetAttackTarget`
  (params (MaxSearchingRange :type "Float (double-precision)") (`Projectile?` :type Boolean) (EnemiesArray :type "Array of /Game/Dynamic/Blueprints/Controllers/Enemies/EnemyBase/BP_Enemy_Base Object Reference (by ref)") (ActorsToIgnore :type "Array of Actor Object Reference (by ref)"))
  (returns (AttackTarget :type "Actor Object Reference"))
  (bind _outhit (`KismetSystemLibrary.LineTraceSingleForObjects` :`Start` (`self.K2_GetActorLocation`) :`End` (`self.K2_GetActorLocation` (`GameplayStatics.GetPlayerCharacter` 0)) :`ObjectTypes` (`|MakeArray` "ObjectTypeQuery1" "ObjectTypeQuery2" "ObjectTypeQuery9" :!type "EObjectTypeQuery Enum") :`DrawDebugType` "ForDuration" :`TraceColor` (struct :`G` 1.0 :`A` 1.0) :`TraceHitColor` (struct :`R` 1.0 :`A` 1.0) :`DrawTime` 0.033333))
  (if (`KismetSystemLibrary.DoesImplementInterface` (`.HitActor` (`GameplayStatics.BreakHitResult` _outhit)) "/Game/Dynamic/Blueprints/Controllers/Player/BPI_Player.BPI_Player_C")
    (return (`GameplayStatics.GetPlayerCharacter` 0))
    (else
      (return null))))

(fn `GetHitReactionMontage`
  (returns (HitReactionMontage :type "AnimMontage Object Reference"))
  (return "/Game/Static/08_Characters/Changelin/AM_changelin_hit_01_Anim.AM_changelin_hit_01_Anim"))

(fn `GetProjectileRange`
  (returns (ProjectileRange :type "Float (double-precision)"))
  (return 0.0))

(fn `UserConstructionScript`
  (`parent.UserConstructionScript`))