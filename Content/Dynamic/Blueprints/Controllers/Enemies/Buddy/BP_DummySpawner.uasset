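; BP_DummySpawner is an actor that spawns BP_Dummy actors at its own transform, starting when play begins.
; Its SpawnDummy event waits briefly, spawns a dummy with itself passed as Spawner, and records it in a tracking array.
; Before spawning, it destroys and removes the oldest tracked dummy if the array's length exceeds MaxDummies.
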(event `self.ReceiveBeginPlay`
  (`self.SpawnDummy`))

(event `SpawnDummy`
  (bind _allspawneddummies (`self.AllSpawnedDummies`))
  (bind _output (`|GetArrayItem` _allspawneddummies))
  (`KismetSystemLibrary.Delay` 2.0)
  (if (> (`KismetArrayLibrary.Array_Length` (`self.AllSpawnedDummies`)) (`self.MaxDummies`))
    (`self.K2_DestroyActor` _output)
    (`KismetArrayLibrary.Array_RemoveItem` _allspawneddummies _output))
  (bind _returnvalue (`|SpawnActorFromClass` "/Game/Dynamic/Blueprints/Controllers/Enemies/Buddy/BP_Dummy.BP_Dummy_C" (`self.GetTransform`) "Undefined" "MultiplyWithRoot" null self null))
  (`KismetArrayLibrary.Array_AddUnique` (`self.AllSpawnedDummies`) _returnvalue))

(fn `UserConstructionScript`)