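; Spawner actor that places melee enemy dummies (BP_Dummy_Melee) at its own transform, starting on BeginPlay.
; SpawnDummy waits briefly, destroys the oldest tracked dummy if the list exceeds MaxDummies, then spawns and records a new one.
; Each dummy receives a speed stat and a reference to the spawner; the spawner itself has no repeat loop.
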(event `self.ReceiveBeginPlay`
  (`self.SpawnDummy`))

(event `self.SpawnDummy`
  (bind _allspawneddummies (`self.AllSpawnedDummies`))
  (bind _output (`|GetArrayItem` _allspawneddummies))
  (`KismetSystemLibrary.Delay` 1.9)
  (if (> (`KismetArrayLibrary.Array_Length` (`self.AllSpawnedDummies`)) (`self.MaxDummies`))
    (`self.K2_DestroyActor` _output)
    (`KismetArrayLibrary.Array_RemoveItem` _allspawneddummies _output))
  (bind _returnvalue (`|SpawnActorFromClass` "/Game/Dynamic/Blueprints/Controllers/Enemies/Dummy/BP_Dummy_Melee.BP_Dummy_Melee_C" (`self.GetTransform`) "Undefined" "MultiplyWithRoot" null self (make `/Game/Dynamic/Blueprints/GameplayAbilitySystem/Effects/Stats/Str_DefaultStats` 100 400.0) null))
  (`KismetArrayLibrary.Array_AddUnique` (`self.AllSpawnedDummies`) _returnvalue))

(fn `UserConstructionScript`)