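; BP_Dummy_Melee is a melee enemy dummy, apparently for testing, that respawns through its Spawner when killed.
; On BeginPlay it assigns its scaling data, marks itself in use at the spawner's transform and prints max health.
; Follow, attack and stat-scaling overrides call parent logic only when their toggles are set.
; It always targets player 0, and on death requests a replacement before destroying itself.
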(event `self.ReceiveBeginPlay`
  (bind _finalstats_maxhealthvalue (break `Str_CharacterStatistics` (`self.FinalStats`)))
  (`parent.ReceiveBeginPlay`)
  (set `self.EnemyScalingData` (`self.EnemyScaling`))
  (`self.SetIsInUse` true (`self.GetTransform` (`self.Spawner`)))
  (`KismetSystemLibrary.PrintString` (`KismetStringLibrary.Conv_IntToString` _finalstats_maxhealthvalue)))

(event `self.ReceiveTick`
  (params (DeltaSeconds :type "Float (single-precision)"))
  (`parent.ReceiveTick` DeltaSeconds))

(event `self.HandleDeath`
  (`/Game/Dynamic/Blueprints/Controllers/Enemies/Dummy/BP_DummyMeleeEliteSpawner.SpawnDummy` (`self.Spawner`))
  (`parent.HandleDeath`)
  (`self.K2_DestroyActor`))

(event `self.FollowPlayer`
  (if (`self.FollowPlayer?`)
    (`parent.FollowPlayer`)))

(event `self.ScaleStatistics`
  (if (`self.ScaleStatistics?`)
    (`parent.ScaleStatistics`)))

(fn `Attack`
  (if (`self.Attack?`)
    (`parent.Attack`)))

(fn `GetAttackRange`
  (returns (AttackRange :type "Float (double-precision)"))
  (return (`self.AttackDistance`)))

(fn `GetAttackTarget`
  (params (MaxSearchingRange :type "Float (double-precision)") (`Projectile?` :type Boolean))
  (returns (AttackTarget :type "Actor Object Reference"))
  (return (`GameplayStatics.GetPlayerCharacter` 0)))

(fn `GetProjectileRange`
  (returns (ProjectileRange :type "Float (double-precision)"))
  (return 0.0))

(fn `UserConstructionScript`)