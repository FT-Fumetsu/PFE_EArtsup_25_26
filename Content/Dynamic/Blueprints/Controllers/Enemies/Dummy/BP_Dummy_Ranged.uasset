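; Ranged dummy enemy, apparently for testing combat, that shows damage taken and respawns through its Spawner on death.
; BeginPlay activates it at the Spawner's transform and listens for an attribute change, spawning BP_DamageIndicator near the neck socket for each decrease.
; Boolean flags gate the parent's attack, player-following and stat-scaling logic, so each behavior can be toggled.
; On death it requests a replacement dummy, runs parent death handling, then destroys itself.
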(event `self.ReceiveBeginPlay`
  (`parent.ReceiveBeginPlay`)
  (set `self.EnemyScalingData` (`self.EnemyScaling`))
  (`self.SetIsInUse` true (`self.GetTransform` (`self.Spawner`)))
  (bind (_asynctaskproxy _attribute _newvalue _oldvalue) (`AbilityAsync_WaitAttributeChanged.WaitForAttributeChanged` null (struct :`AttributeName` "Health" :`Attribute` "/Script/PFE_EArtsup_25_26.BasicAttributeSet:Health" :`AttributeOwner` "/Script/CoreUObject.Class'/Script/PFE_EArtsup_25_26.BasicAttributeSet'"))
    (:`then`
      (`KismetSystemLibrary.Delay` 0.2))
    (:`Changed`
      (if (< _newvalue _oldvalue)
        (bind _returnvalue (- _oldvalue _newvalue))
        (if (!= _returnvalue 0.0)
          (bind (_upvector _rightvector) (message `/Game/Dynamic/Blueprints/FloatingDamage/BPI_PlayerDamageIndicator.GetVectors` (`GameplayStatics.GetPlayerCharacter` 0)))
          (`|SpawnActorFromClass` "/Game/Dynamic/Blueprints/FloatingDamage/BP_DamageIndicator.BP_DamageIndicator_C" (`KismetMathLibrary.MakeTransform` (+ (`SceneComponent.GetSocketLocation` (`self.Mesh`) "neck_02") (* _upvector 20.0) (* _rightvector 20.0))) "Undefined" "MultiplyWithRoot" null _returnvalue null))))))

(event `CustomEvent`
  (params (DeltaSeconds :type "Float (single-precision)"))
  (`parent.ReceiveTick` DeltaSeconds))

(event `self.HandleDeath`
  (`/Game/Dynamic/Blueprints/Controllers/Enemies/Dummy/BP_DummyMeleeEliteSpawner.SpawnDummy` (`self.Spawner`))
  (`parent.HandleDeath`)
  (`self.K2_DestroyActor`))

(event `/Game/Dynamic/Blueprints/Controllers/Enemies/EnemyBase/BaseEnemy/BP_BaseEnemy_Base.FollowPlayer`
  (if (`self.FollowPlayer?`)
    (`parent.FollowPlayer`)))

(event `/Game/Dynamic/Blueprints/Controllers/Enemies/EnemyBase/BaseEnemy/BP_BaseEnemy_Base.ScaleStatistics`
  (if (`self.ScaleStatistics?`)
    (`parent.ScaleStatistics`)))

(fn `Attack`
  (if (`self.Attack?`)
    (`parent.Attack`)))

(fn `UserConstructionScript`
  (`parent.UserConstructionScript`))