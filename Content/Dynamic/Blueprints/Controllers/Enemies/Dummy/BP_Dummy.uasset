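; BP_Dummy is a dummy enemy character that shows damage numbers and respawns through its spawner.
; A Gameplay Ability System attribute listener spawns a BP_DamageIndicator with the amount lost on each decrease, offset from the neck socket along player-provided up and right vectors.
; On death it asks the Spawner for a new dummy before running parent handling.
; Attack overrides return zero ranges and target the player.
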(event `self.ReceiveBeginPlay`
  (bind (_asynctaskproxy _attribute _newvalue _oldvalue) (`AbilityAsync_WaitAttributeChanged.WaitForAttributeChanged` null (struct :`AttributeName` "Health" :`Attribute` "/Script/PFE_EArtsup_25_26.BasicAttributeSet:Health" :`AttributeOwner` "/Script/CoreUObject.Class'/Script/PFE_EArtsup_25_26.BasicAttributeSet'"))
    (:`then`
      (`KismetSystemLibrary.Delay` 0.2))
    (:`Changed`
      (if (< _newvalue _oldvalue)
        (bind _returnvalue (- _oldvalue _newvalue))
        (if (!= _returnvalue 0.0)
          (bind (_upvector _rightvector) (message `/Game/Dynamic/Blueprints/FloatingDamage/BPI_PlayerDamageIndicator.GetVectors` (`GameplayStatics.GetPlayerCharacter` 0)))
          (`|SpawnActorFromClass` "/Game/Dynamic/Blueprints/FloatingDamage/BP_DamageIndicator.BP_DamageIndicator_C" (`KismetMathLibrary.MakeTransform` (+ (`SceneComponent.GetSocketLocation` (`self.Mesh`) "neck_02") (* _upvector 20.0) (* _rightvector 20.0))) "Undefined" "MultiplyWithRoot" null _returnvalue null))))))

(event `self.HandleDeath`
  (`/Game/Dynamic/Blueprints/Controllers/Enemies/Dummy/BP_DummySpawner.SpawnDummy` (`self.Spawner`))
  (`parent.HandleDeath`))

(fn `GetAttackRange`
  (returns (AttackRange :type "Float (double-precision)"))
  (return 0.0))

(fn `GetAttackTarget`
  (params (MaxSearchingRange :type "Float (double-precision)") (`Projectile?` :type Boolean))
  (returns (AttackTarget :type "Actor Object Reference"))
  (return (`GameplayStatics.GetPlayerCharacter` 0)))

(fn `GetProjectileRange`
  (returns (ProjectileRange :type "Float (double-precision)"))
  (return 0.0))

(fn `UserConstructionScript`)