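; Spawner actor that places melee training dummies (BP_Dummy_Melee) at its own transform, optionally as elites with boosted stats.
; SpawnDummy runs on BeginPlay, waits briefly, then destroys the oldest tracked dummy if the list exceeds MaxDummies.
; When Elite is set, a collapsed graph scales the default stats by StatsMultiplier.
; Each new dummy receives the final stats and a reference to the spawner, then joins the tracked list.
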(event `self.ReceiveBeginPlay`
  (`self.SpawnDummy`))

(event `self.SpawnDummy`
  (bind _allspawneddummies (`self.AllSpawnedDummies`))
  (bind _output (`|GetArrayItem` _allspawneddummies))
  (`KismetSystemLibrary.Delay` 1.9)
  (set `self.FinalStats` (`self.Default Stats Struct`))
  (if (> (`KismetArrayLibrary.Array_Length` (`self.AllSpawnedDummies`)) (`self.MaxDummies`))
    (`self.K2_DestroyActor` _output)
    (`KismetArrayLibrary.Array_RemoveItem` _allspawneddummies _output))
  (if (`self.Elite?`)
    (`self.StatsMultiplierWhenElite`
      (:`Out`
        _)))
  (bind _returnvalue (`|SpawnActorFromClass` "/Game/Dynamic/Blueprints/Controllers/Enemies/Dummy/BP_Dummy_Melee.BP_Dummy_Melee_C" (`self.GetTransform`) "Undefined" "MultiplyWithRoot" null self (`self.FinalStats`) null))
  (`KismetArrayLibrary.Array_AddUnique` (`self.AllSpawnedDummies`) _returnvalue))

(fn `UserConstructionScript`)