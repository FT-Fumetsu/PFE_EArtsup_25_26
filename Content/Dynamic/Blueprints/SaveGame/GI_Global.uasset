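; Game instance that owns the game's settings save object, loading it on Init and exposing it through GetGame.
; Save and load each support synchronous or async slot operations, and SaveSettings writes new settings into the object before saving.
; When no save exists, it creates a fresh SG_Settings object in memory and applies windowed, 1080p, lowest-scalability defaults through GameUserSettings.
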(event `self.ReceiveInit`
  (`/Game/Dynamic/Blueprints/SaveGame/BPI_SaveGame.LoadGame` false))

(event `/Game/Dynamic/Blueprints/SaveGame/BPI_SaveGame.SaveGame`
  (params (Async :type Boolean))
  ; Save Game
  (if Async
    (`AsyncActionHandleSaveGame.AsyncSaveGameToSlot` (`self.SettingsSaveGame`) (`self.Slot Name`))
    (else
      (`GameplayStatics.SaveGameToSlot` (`self.SettingsSaveGame`) (`self.Slot Name`)))))

(event `/Game/Dynamic/Blueprints/SaveGame/BPI_SaveGame.LoadGame`
  (params (Async :type Boolean))
  ; Load Game
  (bind _returnvalue (`GameplayStatics.DoesSaveGameExist` (`self.Slot Name`)))
  (if _returnvalue
    (if Async
      (bind _savegame (`AsyncActionHandleSaveGame.AsyncLoadGameFromSlot` (`self.Slot Name`))
        (:`then`
          (bind _assg_settings (cast `/Game/Dynamic/Blueprints/SaveGame/SG_Settings` _savegame))
          (set `self.SettingsSaveGame` _assg_settings)))
      (else
        (bind _returnvalue_2 (`GameplayStatics.LoadGameFromSlot` (`self.Slot Name`)))
        (bind _assg_settings_2 (cast `/Game/Dynamic/Blueprints/SaveGame/SG_Settings` _returnvalue_2))
        (set `self.SettingsSaveGame` _assg_settings_2)))
    (else
      (bind _returnvalue_3 (`GameplayStatics.CreateSaveGameObject` "/Game/Dynamic/Blueprints/SaveGame/SG_Settings.SG_Settings_C"))
      (set `self.SettingsSaveGame` _returnvalue_3)
      (bind _returnvalue_4 (`GameUserSettings.GetGameUserSettings`))
      (`GameUserSettings.SetFullscreenMode` _returnvalue_4 "Windowed")
      (`GameUserSettings.SetScreenResolution` _returnvalue_4 (make `IntPoint` 1920 1080))
      (`GameUserSettings.SetOverallScalabilityLevel` _returnvalue_4 0)
      (`GameUserSettings.ApplySettings` _returnvalue_4 true))))

(event `/Game/Dynamic/Blueprints/SaveGame/BPI_SaveGame.SaveSettings`
  (params (SettingsSave :type "/Game/Dynamic/Blueprints/SaveGame/Str_SaveSettings Structure") (Async :type Boolean))
  (set `/Game/Dynamic/Blueprints/SaveGame/SG_Settings.SaveSettings` SettingsSave (`self.SettingsSaveGame`))
  (`self.SaveGame` Async))

(fn `GetGame`
  (returns (SettingsSave :type "/Game/Dynamic/Blueprints/SaveGame/SG_Settings Object Reference"))
  (return (`self.SettingsSaveGame`)))