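; Narrative component that steps through data-table dialogue in a WBP_Dialogue widget.
; Each Interact creates or updates the widget from the current row, which supplies the next row, table and end flag.
; Leaving, or interacting after the end, removes the widget, restores game input, unpauses and clears the player's DialogueLauncher.
; That exit also saves settings with the tutorial marked finished and opens the BlockoutLondon_Duplicated level.
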(event `/Game/Dynamic/Blueprints/DialogueSystem/Interfaces/BPI_NarrativeInterface.LeaveDialogue`
  (bind _returnvalue (`GameplayStatics.GetGameInstance`))
  (bind _returnvalue_2 (`GameplayStatics.GetPlayerController` 0))
  (`/Engine/EditorBlueprintResources/StandardMacros.IsValid` (`self.DialogueWidget`)
    (:`Is Valid`
      (`Widget.RemoveFromParent` (`self.DialogueWidget`) :!label _label)
      (set `self.EndDialogue?` false)
      (set `self.DialogueWidget` null)
      (`WidgetBlueprintLibrary.SetInputMode_GameOnly` _returnvalue_2)
      (set `PlayerController.bShowMouseCursor` false _returnvalue_2)
      (`GameplayStatics.SetGamePaused` false)
      (set `self.DialogueLauched` false)
      (bind _asbp_player (cast `/Game/Dynamic/Blueprints/Controllers/Player/BP_Player` (`GameplayStatics.GetPlayerCharacter` 0)))
      (set `/Game/Dynamic/Blueprints/Controllers/Player/BP_Player.DialogueLauncher` null _asbp_player)
      (bind _settingssave (message `/Game/Dynamic/Blueprints/SaveGame/BPI_SaveGame.GetGame` _returnvalue))
      (bind (_savesettings_mastervolume _savesettings_musicvolume _savesettings_sfxvolume _savesettings_gammavalue) (break `/Game/Dynamic/Blueprints/SaveGame/Str_SaveSettings` (`/Game/Dynamic/Blueprints/SaveGame/SG_Settings.SaveSettings` _settingssave)))
      (message `/Game/Dynamic/Blueprints/SaveGame/BPI_SaveGame.SaveSettings` _returnvalue (make `/Game/Dynamic/Blueprints/SaveGame/Str_SaveSettings` _savesettings_mastervolume _savesettings_musicvolume _savesettings_sfxvolume _savesettings_gammavalue true) false)
      (`GameplayStatics.OpenLevelBySoftObjectPtr` "/Game/Dynamic/Levels/DevLevels/Blockout-London_Duplicated.Blockout-London_Duplicated"))))

(event `/Game/Dynamic/Blueprints/DialogueSystem/Interfaces/BPI_NarrativeInterface.Interact`
  (bind _returnvalue (`GameplayStatics.GetPlayerController` 0))
  (if (`self.EndDialogue?`)
    (goto _label)
    (else
      (`/Engine/EditorBlueprintResources/StandardMacros.IsValid` (`self.DialogueWidget`)
        (:`Is Valid`
          (bind _returnvalue_2 (`|GetDataTableRow` (`self.Data Table`) (`self.Row Name`))
            (:`then`
              (bind (_speakername _dialogue _speakericon _nextrowname _datatable _enddialogue_) (break `/Game/Dynamic/Blueprints/DialogueSystem/Structure/Str_Dialogue` _returnvalue_2))
              (`/Game/Dynamic/Blueprints/DialogueSystem/Widgets/WBP_Dialogue.UpdateDialogue` (`self.DialogueWidget`) _speakername _dialogue _speakericon)
              (set `self.Row Name` _nextrowname)
              (set `self.Data Table` _datatable)
              (set `self.EndDialogue?` _enddialogue_))))
        (:`Is Not Valid`
          (bind _returnvalue_3 (`|GetDataTableRow` (`self.Data Table`) (`self.Row Name`))
            (:`then`
              (bind (_speakername_2 _dialogue_2 _speakericon_2 _nextrowname_2 _datatable_2 _enddialogue__2) (break `/Game/Dynamic/Blueprints/DialogueSystem/Structure/Str_Dialogue` _returnvalue_3))
              (bind _returnvalue_4 (`|CreateWidget` "/Game/Dynamic/Blueprints/DialogueSystem/Widgets/WBP_Dialogue.WBP_Dialogue_C" null _speakername_2 _dialogue_2 _speakericon_2))
              (bind _output_get (set `self.DialogueWidget` _returnvalue_4))
              (`UserWidget.AddToViewport` _output_get 0)
              (set `self.Row Name` _nextrowname_2)
              (set `self.Data Table` _datatable_2)
              (set `self.EndDialogue?` _enddialogue__2)
              (`WidgetBlueprintLibrary.SetInputMode_GameAndUIEx` _returnvalue null)
              (set `PlayerController.bShowMouseCursor` true _returnvalue))))))))