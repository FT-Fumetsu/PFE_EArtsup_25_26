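; Game flow manager that runs data-table-driven enemy waves and includes a time-threshold check for game phases.
; BeginSpawns caches the row names and, after a short delay, loads the first wave, which sets a looping spawn timer and, unless flagged End, a timer for NextWave.
; SpawnEnemies pulls random enemy classes from a pool manager.
; NextWave clears all timers and advances the index, holding it short of the last row.
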(event `BeginSpawns`
  (`self.SetActorTickEnabled` true)
  (bind _outrownames (`DataTableFunctionLibrary.GetDataTableRowNames` (`self.SpawnDataTable`)))
  (set `self.RowNames` _outrownames)
  (set `self.CurrentWaveIndex` 0)
  (`KismetSystemLibrary.Delay` 5.0)
  (`self.LoadWave`))

(event `LoadWave`
  (bind ((`SpawnInterval_4_B286F7EE486F2FF6F67C0FB283A72E5C` _spawninterval) (`TimeBeforeChangingSpawn_6_B1444D1B40299164A9CAA4A5F983E28C` _timebeforechangingspawn) (`End?_9_280F9CFE43D29DEF1D54FCB629494914` _end_)) (break `/Game/Dynamic/Blueprints/WaveSystem/Str_Spawn` (`self.CurrentWaveData`)))
  (bind _returnvalue (`|GetDataTableRow` (`self.SpawnDataTable`) (`|GetArrayItem` (`self.RowNames`) (`self.CurrentWaveIndex`)))
    (:`then`
      (set `self.CurrentWaveData` _returnvalue)
      (if (not _end_)
        (bind _returnvalue_2 (`KismetSystemLibrary.K2_SetTimerDelegate` (delegate `NextWave`) _timebeforechangingspawn))
        (`KismetArrayLibrary.Array_AddUnique` (`self.AllTimers`) _returnvalue_2))
      (bind _returnvalue_3 (`KismetSystemLibrary.K2_SetTimerDelegate` (`|CreateDelegate` :!event `SpawnEnemies`) _spawninterval true))
      (`KismetArrayLibrary.Array_AddUnique` (`self.AllTimers`) _returnvalue_3))))

(event `SpawnEnemies`
  (for _ (range (`.EnemyCount_10_B826C1254E0DDC5E737AF2B9357FB53D` (break `/Game/Dynamic/Blueprints/WaveSystem/Str_Spawn` (`self.CurrentWaveData`))))
    (`/Game/Dynamic/Blueprints/ObjectPool/Enemy/BP_EnemiesPoolManager.SpawnEnemyFromPool` (`self.EnemiesPoolManager`) (`KismetArrayLibrary.Array_Random` (`self.EnemiesClasses`)))))

(event `NextWave`
  (for _array_element (`self.AllTimers`)
    (`KismetSystemLibrary.K2_ClearAndInvalidateTimerHandle` _array_element))
  (`KismetArrayLibrary.Array_Clear` (`self.AllTimers`))
  (bind _output_get (set `self.CurrentWaveIndex` (+ (`self.CurrentWaveIndex`) 1)))
  (if (not (< _output_get (- (`KismetArrayLibrary.Array_Length` (`self.RowNames`)) 1)))
    (set `self.CurrentWaveIndex` (- (`self.CurrentWaveIndex`) 1)))
  (`self.LoadWave`))

(fn `UserConstructionScript`)