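; BP_OcclusionShader is an occlusion Blueprint that makes components overlapping its StaticMesh see-through.
; Begin overlap swaps every material slot to dynamic MAT_Occlusion instances at low Opacity, caching them per component in OcclusionDataArray for reuse.
; Original materials are never restored.
; End overlap sets cached instances to that same low Opacity, so they stay faded; only uncached components get new, fully opaque instances.
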(event `self.StaticMesh.OnComponentBeginOverlap`
  (params (OverlappedComponent :type "PrimitiveComponent Object Reference") (OtherActor :type "Actor Object Reference") (OtherComp :type "PrimitiveComponent Object Reference") (OtherBodyIndex :type Integer) (bFromSweep :type Boolean) (SweepResult :type "HitResult Structure (by ref)"))
  (bind (_currentocclusiondata_mesh _currentocclusiondata_materials) (break `/Game/Dynamic/Blueprints/Shader/Str_OcclusionData` (`self.CurrentOcclusionData`)))
  (bind (_currentocclusiondata_mesh_2 _currentocclusiondata_materials_2) (break `/Game/Dynamic/Blueprints/Shader/Str_OcclusionData` (`self.CurrentOcclusionData`)))
  (for _array_element (`self.OcclusionDataArray`)
    (if (== (`.Mesh_2_2541833B4E6253CD24F7A9AC5CB59948` (break `/Game/Dynamic/Blueprints/Shader/Str_OcclusionData` _array_element)) OtherComp)
      (set `self.Found` true)
      (set `self.CurrentOcclusionData` _array_element)
      (break)))
  (if (`self.Found`)
    (for _array_element_2 _currentocclusiondata_materials
      (`MaterialInstanceDynamic.SetScalarParameterValue` _array_element_2 "Opacity" 0.3))
    (else
      (set `self.CurrentOcclusionData` (make `/Game/Dynamic/Blueprints/Shader/Str_OcclusionData` OtherComp))
      (for _index (range (`PrimitiveComponent.GetNumMaterials` OtherComp))
        (bind _returnvalue (`PrimitiveComponent.CreateDynamicMaterialInstance` OtherComp _index "/Game/Static/02_Materials/Dev/MAT_Occlusion.MAT_Occlusion" "None"))
        (`KismetArrayLibrary.Array_AddUnique` _currentocclusiondata_materials_2 _returnvalue)
        (`MaterialInstanceDynamic.SetScalarParameterValue` _returnvalue "Opacity" 0.3))
      (`KismetArrayLibrary.Array_AddUnique` (`self.OcclusionDataArray`) (`self.CurrentOcclusionData`)))))

(event `self.StaticMesh.OnComponentEndOverlap`
  (params (OverlappedComponent :type "PrimitiveComponent Object Reference") (OtherActor :type "Actor Object Reference") (OtherComp :type "PrimitiveComponent Object Reference") (OtherBodyIndex :type Integer))
  (bind (_currentocclusiondata_mesh _currentocclusiondata_materials) (break `/Game/Dynamic/Blueprints/Shader/Str_OcclusionData` (`self.CurrentOcclusionData`)))
  (for _array_element (`self.OcclusionDataArray`)
    (if (== (`.Mesh_2_2541833B4E6253CD24F7A9AC5CB59948` (break `/Game/Dynamic/Blueprints/Shader/Str_OcclusionData` _array_element)) OtherComp)
      (set `self.Found` true)
      (set `self.CurrentOcclusionData` _array_element)
      (break)))
  (if (`self.Found`)
    (for _array_element_2 _currentocclusiondata_materials
      (`MaterialInstanceDynamic.SetScalarParameterValue` _array_element_2 "Opacity" 0.3))
    (else
      (for _index (range (`PrimitiveComponent.GetNumMaterials` OtherComp))
        (bind _returnvalue (`PrimitiveComponent.CreateDynamicMaterialInstance` OtherComp _index "/Game/Static/02_Materials/Dev/MAT_Occlusion.MAT_Occlusion" "None"))
        (`MaterialInstanceDynamic.SetScalarParameterValue` _returnvalue "Opacity" 1.0)))))

(fn `UserConstructionScript`)