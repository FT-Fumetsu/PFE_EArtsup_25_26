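; Floating damage indicator actor that shows a damage value in a widget and drifts away from its spawn point before disappearing.
; On BeginPlay it passes Damage to its DamageWidget and picks a randomized end point up and to the right, using vectors supplied by the player character.
; A timeline interpolates the actor to that point, then destroys it when finished.
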(event `self.ReceiveBeginPlay`
  (message `/Game/Dynamic/Blueprints/FloatingDamage/BPI_DamageIndicator.SetDamage` (`WidgetComponent.GetWidget` (`self.DamageWidget`)) (`self.Damage`))
  (bind _output_get (set `self.StartPosition` (`self.K2_GetActorLocation`)))
  (bind (_upvector _rightvector) (message `/Game/Dynamic/Blueprints/FloatingDamage/BPI_PlayerDamageIndicator.GetVectors` (`GameplayStatics.GetPlayerCharacter` 0)))
  (set `self.EndPosition` (+ _output_get (* _upvector (`KismetMathLibrary.RandomFloatInRange` 40.0 50.0)) (* _rightvector (`KismetMathLibrary.RandomFloatInRange` 20.0 30.0))))
  (bind (_direction _newtrack_0) (`Timeline|Timeline`)
    (:`Update`
      (`self.K2_SetActorLocation` (`KismetMathLibrary.VLerp` (`self.StartPosition`) (`self.EndPosition`) _newtrack_0)))
    (:`Finished`
      (`self.K2_DestroyActor`))))

(fn `UserConstructionScript`)